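; BP_FallingStone is a stone that starts falling when the third-person character overlaps its CheckPlayerCollision trigger.
; Tick then moves it down by a randomized per-frame step, unscaled by delta time and without sweep, and destroys it below a Z threshold.
; RockCollision overlapping a BP_StoneBox plays a smoke sound and sets a ComponentCollision flag, which a StoneBox overlap on the trigger clears; this graph never reads the flag.
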(event `self.ReceiveBeginPlay`
  (set `self.Gravity` -5.0))

(event `self.ReceiveTick`
  (params (DeltaSeconds :type "Float (single-precision)"))
  (bind (_returnvalue_x _returnvalue_y _returnvalue_z) (`KismetMathLibrary.BreakVector` (`self.K2_GetActorLocation`)))
  (bind _returnvalue (+ (`self.Gravity`) (`KismetMathLibrary.RandomFloatInRange` -3.0 -6.0)))
  (if (`self.Check Player`)
    (`self.K2_SetActorLocation` (+ (`self.K2_GetActorLocation`) (`KismetMathLibrary.MakeVector` 0.0 0.0 _returnvalue)))
    (if (< _returnvalue_z -2000.0)
      (`self.K2_DestroyActor`)
      (set `self.Gravity` _returnvalue))))

(event `self.RockCollision.OnComponentBeginOverlap`
  (params (OverlappedComponent :type "PrimitiveComponent Object Reference") (OtherActor :type "Actor Object Reference") (OtherComp :type "PrimitiveComponent Object Reference") (OtherBodyIndex :type Integer) (bFromSweep :type Boolean) (SweepResult :type "HitResult Structure (by ref)"))
  (cast `/Game/GE_BluePrint/BP_StoneBox` OtherActor)
  (set `self.Component Collision` true)
  (`GameplayStatics.PlaySound2D` "/Game/StarterContent/Audio/Smoke01.Smoke01" 1.0 1.0 0.0 null null))

(event `self.CheckPlayerCollision.OnComponentBeginOverlap`
  (params (OverlappedComponent :type "PrimitiveComponent Object Reference") (OtherActor :type "Actor Object Reference") (OtherComp :type "PrimitiveComponent Object Reference") (OtherBodyIndex :type Integer) (bFromSweep :type Boolean) (SweepResult :type "HitResult Structure (by ref)"))
  (cast `/Game/GE_BluePrint/BP_StoneBox` OtherActor
    (:`then`
      (set `self.Component Collision` false))
    (:`CastFailed`
      _))
  (cast `/Game/ThirdPerson/Blueprints/BP_ThirdPersonCharacter` OtherActor)
  (set `self.Check Player` true))

(fn `UserConstructionScript`)