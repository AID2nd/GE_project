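; BP_Potion is a potion pickup that flies to the player like a magnet and then destroys itself.
; Its collision box stores the overlapping third-person character and flags it in range, clearing the flag on exit.
; While flagged, Tick calls CheckPlayerHP, which only checks that the player isn't falling before playing the Magnet timeline.
; The timeline lerps the potion toward the player, with destruction after a short delay; no healing happens here.
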(event `self.ReceiveTick`
  (params (DeltaSeconds :type "Float (single-precision)"))
  (if (`self.Is Player In Area?`)
    (`self.Check Player HP`)))

(event `self.ItemCollisionBox.OnComponentBeginOverlap`
  (params (OverlappedComponent :type "PrimitiveComponent Object Reference") (OtherActor :type "Actor Object Reference") (OtherComp :type "PrimitiveComponent Object Reference") (OtherBodyIndex :type Integer) (bFromSweep :type Boolean) (SweepResult :type "HitResult Structure (by ref)"))
  (bind _asbp_third_person_character (cast `/Game/ThirdPerson/Blueprints/BP_ThirdPersonCharacter` OtherActor))
  (set `self.Player` _asbp_third_person_character)
  (set `self.Is Player In Area?` true))

(event `self.ItemCollisionBox.OnComponentEndOverlap`
  (params (OverlappedComponent :type "PrimitiveComponent Object Reference") (OtherActor :type "Actor Object Reference") (OtherComp :type "PrimitiveComponent Object Reference") (OtherBodyIndex :type Integer))
  (set `self.Is Player In Area?` false))

(event `Check Player HP`
  (if (not (`NavMovementComponent.IsFalling` (`Character.CharacterMovement` (`self.Player`))))
    (bind (_direction _newtrack_0) (`Timeline|Magnet`)
      (:`Update`
        (`self.K2_SetActorLocation` (`KismetMathLibrary.VLerp` (`self.K2_GetActorLocation`) (`self.K2_GetActorLocation` (`self.Player`)) _newtrack_0))
        (`KismetSystemLibrary.Delay` 0.5)
        (`self.K2_DestroyActor`)))))

(fn `UserConstructionScript`)