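; A pressure button Blueprint, named for a thorn wall, that sinks while its Box is overlapped and rises back when the overlap ends.
; BeginPlay records the resting Z height and picks one of two paint materials from MaterialNumber.
; Box overlap events set PlayerOnButton without filtering the actor, and Tick moves the actor in fixed per-frame steps, independent of delta time.
; The file contains no link to a wall.
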(event `self.ReceiveBeginPlay`
  (bind (_returnvalue_x _returnvalue_y _returnvalue_z) (`KismetMathLibrary.BreakVector` (`self.K2_GetActorLocation`)))
  (bind _staticmeshcomponent (`self.StaticMeshComponent`))
  (bind _staticmeshcomponent_2 (`self.StaticMeshComponent`))
  (set `self.Button Location` _returnvalue_z)
  (switch `int` (`self.Material Number`)
    (:`0`
      (`PrimitiveComponent.SetMaterial` _staticmeshcomponent_2 0 "/Game/Assets/Material/MM_Paint1.MM_Paint1")
      (`PrimitiveComponent.SetMaterial` _staticmeshcomponent_2 1 "/Game/Assets/Material/MM_Paint1.MM_Paint1"))
    (:`1`
      (`PrimitiveComponent.SetMaterial` _staticmeshcomponent 0 "/Game/Assets/Material/MM_Paint2.MM_Paint2")
      (`PrimitiveComponent.SetMaterial` _staticmeshcomponent 1 "/Game/Assets/Material/MM_Paint2.MM_Paint2"))))

(event `self.ReceiveActorBeginOverlap`
  (params (OtherActor :type "Actor Object Reference")))

(event `self.ReceiveTick`
  (params (DeltaSeconds :type "Float (single-precision)"))
  (bind (_returnvalue_x _returnvalue_y _returnvalue_z) (`KismetMathLibrary.BreakVector` (`self.K2_GetActorLocation`)))
  (bind (_returnvalue_x_2 _returnvalue_y_2 _returnvalue_z_2) (`KismetMathLibrary.BreakVector` (`self.K2_GetActorLocation`)))
  (if (`self.Player On Button?`)
    (if (not (> (- (`self.Button Location`) _returnvalue_z_2) 20.0))
      (`self.K2_SetActorLocation` (+ (`self.K2_GetActorLocation`) (0.0 0.0 -1.0))))
    (elif (> (- (`self.Button Location`) _returnvalue_z) 0.0)
      (`self.K2_SetActorLocation` (+ (`self.K2_GetActorLocation`) (0.0 0.0 1.0))))))

(event `self.Box.OnComponentBeginOverlap`
  (params (OverlappedComponent :type "PrimitiveComponent Object Reference") (OtherActor :type "Actor Object Reference") (OtherComp :type "PrimitiveComponent Object Reference") (OtherBodyIndex :type Integer) (bFromSweep :type Boolean) (SweepResult :type "HitResult Structure (by ref)"))
  (set `self.Player On Button?` true))

(event `self.Box.OnComponentEndOverlap`
  (params (OverlappedComponent :type "PrimitiveComponent Object Reference") (OtherActor :type "Actor Object Reference") (OtherComp :type "PrimitiveComponent Object Reference") (OtherBodyIndex :type Integer))
  (set `self.Player On Button?` false))

(fn `UserConstructionScript`)