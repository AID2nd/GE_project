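; BladeBP is the playable sword character, with movement, dash, jump, three-hit combo, timed guard and two relic-gated MP skills.
; Animation-driven events chain combos and toggle hit capsules, whose overlaps apply damage to differently tagged characters.
; Damage updates the GameInstance's HUD and can trigger one revive that flags HellDemonBP and Aiblade.
; Tick polls flags for final death with per-stage fail screens, relic HP/attack bonuses and guard cooldown.
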(event `부활`
  (`KismetSystemLibrary.Delay` 1.5)
  (set `self.IsDeath` false)
  (set `self.Hp` 200.0)
  (`/Game/Blueprints/Widgets/GamePlayMainWidget.Update_HeroHPBar` (`/Game/Blueprints/SideScrollGameInstance.gwmg` (`self.SideScrollGameInsRef`)) (`self.Hp`) (`self.MaxHp`))
  (set `self.Mp` 100.0)
  (`/Game/Blueprints/Widgets/GamePlayMainWidget.Update_MPBar` (`/Game/Blueprints/SideScrollGameInstance.gwmg` (`self.SideScrollGameInsRef`)) (`self.Mp`) (`self.MaxMp`))
  (bind _returnvalue (`GameplayStatics.GetActorOfClass` "/Game/HellDemonBoss/HellDemonBP.HellDemonBP_C"))
  (set `/Game/HellDemonBoss/HellDemonBP.isAiDie` true _returnvalue))

(event `self.ReceiveTick`
  (params (DeltaSeconds :type "Float (single-precision)"))
  (bind _returnvalue (`GameplayStatics.GetPlayerController` 0))
  (bind _returnvalue_2 (`GameplayStatics.GetPlayerController` 0))
  (bind _returnvalue_3 (`GameplayStatics.GetPlayerController` 0))
  (bind _returnvalue_4 (`GameplayStatics.GetPlayerController` 0))
  (`|ExecutionSequence`
    (:`then_0`
      (if (`self.IsDeath`)
        (`|ExecutionSequence`
          (:`then_0`
            (if (`self.isbossStage1`)
              (`/Engine/EditorBlueprintResources/StandardMacros.DoOnce` false
                (:`Completed`
                  (`WidgetLayoutLibrary.RemoveAllWidgets`)
                  (`self.PlayAnimMontage` "/Game/BLADE/montage/BLADE_DEATH_Montage.BLADE_DEATH_Montage")
                  (`KismetSystemLibrary.Delay` 1.0)
                  (`ActorComponent.K2_DestroyComponent` (`self.Mesh`))
                  (bind _returnvalue_5 (`|CreateWidget` "/Game/Blueprints/Widgets/StageFail_BossRoom.StageFail_BossRoom_C" _returnvalue_2))
                  (`UserWidget.AddToViewport` _returnvalue_5 0)
                  (set `PlayerController.bShowMouseCursor` true _returnvalue_2)
                  (`self.DisableInput` (`GameplayStatics.GetPlayerCharacter` 0) (`GameplayStatics.GetPlayerController` 0))))))
          (:`then_1`
            (if (`self.isBossStage2`)
              (`/Engine/EditorBlueprintResources/StandardMacros.DoOnce` false
                (:`Completed`
                  (`WidgetLayoutLibrary.RemoveAllWidgets`)
                  (`self.PlayAnimMontage` "/Game/BLADE/montage/BLADE_DEATH_Montage.BLADE_DEATH_Montage")
                  (`KismetSystemLibrary.Delay` 1.5)
                  (`ActorComponent.K2_DestroyComponent` (`self.Mesh`))
                  (bind _returnvalue_6 (`|CreateWidget` "/Game/Blueprints/Widgets/FinalStageFail.FinalStageFail_C" _returnvalue))
                  (`UserWidget.AddToViewport` _returnvalue_6 0)
                  (set `PlayerController.bShowMouseCursor` true _returnvalue)
                  (`self.DisableInput` (`GameplayStatics.GetPlayerCharacter` 0) (`GameplayStatics.GetPlayerController` 0))))))
          (:`then_2`
            (if (`self.isStage2`)
              (`/Engine/EditorBlueprintResources/StandardMacros.DoOnce` false
                (:`Completed`
                  (`WidgetLayoutLibrary.RemoveAllWidgets`)
                  (`self.PlayAnimMontage` "/Game/BLADE/montage/BLADE_DEATH_Montage.BLADE_DEATH_Montage")
                  (`KismetSystemLibrary.Delay` 1.0)
                  (`ActorComponent.K2_DestroyComponent` (`self.Mesh`))
                  (bind _returnvalue_7 (`|CreateWidget` "/Game/Blueprints/Widgets/2StageFail.2StageFail_C" _returnvalue_3))
                  (`UserWidget.AddToViewport` _returnvalue_7 0)
                  (set `PlayerController.bShowMouseCursor` true _returnvalue_3)
                  (`self.DisableInput` (`GameplayStatics.GetPlayerCharacter` 0) (`GameplayStatics.GetPlayerController` 0))))))
          (:`then_3`
            (if (`self.isfield`)
              (`/Engine/EditorBlueprintResources/StandardMacros.DoOnce` false
                (:`Completed`
                  (`WidgetLayoutLibrary.RemoveAllWidgets`)
                  (`self.PlayAnimMontage` "/Game/BLADE/montage/BLADE_DEATH_Montage.BLADE_DEATH_Montage")
                  (`KismetSystemLibrary.Delay` 1.0)
                  (`ActorComponent.K2_DestroyComponent` (`self.Mesh`))
                  (bind _returnvalue_8 (`|CreateWidget` "/Game/Blueprints/Widgets/StageFail.StageFail_C" _returnvalue_4))
                  (`UserWidget.AddToViewport` _returnvalue_8 0)
                  (set `PlayerController.bShowMouseCursor` true _returnvalue_4)
                  (`self.DisableInput` (`GameplayStatics.GetPlayerCharacter` 0) (`GameplayStatics.GetPlayerController` 0)))))))))
    (:`then_1`
      (if (>= (`self.grailCount`) 1.0)
        (`/Engine/EditorBlueprintResources/StandardMacros.DoOnce` false
          (:`Completed`
            (set `self.MaxHp` 300.0)
            (set `self.Hp` (+ (`self.Hp`) 100.0))))))
    (:`then_2`
      (if (>= (`self.SkullCount`) 1.0)
        (`/Engine/EditorBlueprintResources/StandardMacros.DoOnce` false
          (:`Completed`
            (set `self.Atk` 30.0)))))
    (:`then_3`
      (if (`self.isgTimer`)
        (`self.guardTimer`)))
    (:`then_4`
      (if (`self.isSussNorGuard`)
        (if (`self.isNodamage`)
          (`KismetSystemLibrary.PrintString` "한손공격방어성공")
          (set `self.isSussNorGuard` false))))
    (:`then_5`
      (if (`self.isBSkiAttack`)
        (`KismetSystemLibrary.PrintString` "양손공격")
        (set `self.isBSkiAttack` false)))))

(event `self.ReceiveBeginPlay`
  (bind _asside_scroll_game_instance (cast `/Game/Blueprints/SideScrollGameInstance` (`GameplayStatics.GetGameInstance`)))
  (set `self.SideScrollGameInsRef` _asside_scroll_game_instance)
  (set `self.isSave` false)
  (set `self.isPendent` false)
  (set `self.ismove` true)
  (set `self.Hp` 200.0)
  (`/Game/Blueprints/Widgets/GamePlayMainWidget.Update_HeroHPBar` (`/Game/Blueprints/SideScrollGameInstance.gwmg` (`self.SideScrollGameInsRef`)) (`self.Hp`) (`self.MaxHp`))
  (set `self.Mp` 100.0)
  (`/Game/Blueprints/Widgets/GamePlayMainWidget.Update_MPBar` (`/Game/Blueprints/SideScrollGameInstance.gwmg` (`self.SideScrollGameInsRef`)) (`self.Mp`) (`self.MaxMp`))
  (set `self.isNodamage` false))

(event `heal`
  (if (`self.is heal`)
    (set `self.Hp` (+ (`self.Hp`) 10.0))
    (`/Game/Blueprints/Widgets/GamePlayMainWidget.Update_HeroHPBar` (`/Game/Blueprints/SideScrollGameInstance.gwmg` (`self.SideScrollGameInsRef`)) (`self.Hp`) (`self.MaxHp`))
    (set `self.is heal` false)))

(event `MpHeal`
  (if (`self.ismpHeal`)
    (set `self.Mp` (+ (`self.Mp`) 10.0))
    (`/Game/Blueprints/Widgets/GamePlayMainWidget.Update_MPBar` (`/Game/Blueprints/SideScrollGameInstance.gwmg` (`self.SideScrollGameInsRef`)) (`self.Mp`) (`self.MaxMp`))
    (set `self.ismpHeal` false)))

(event `InputAxis|LeftRight`
  (params (AxisValue :type "Float (single-precision)"))
  (if (`self.ismove`)
    (if (not (`self.IsAttacking`))
      (`SceneComponent.SetHiddenInGame` (`self.Slash`) true true)
      (`self.AddMovementInput` (`KismetMathLibrary.GetRightVector` (`KismetMathLibrary.MakeRotator` 0.0 0.0 (.yaw (`self.GetControlRotation`)))) AxisValue))))

(event `Key|LeftShift`
  (params (Key :type "Key Structure"))
  (bind _returnvalue (`self.GetActorForwardVector`))
  (:`Pressed`
    (if (>= (`self.DashCoolDown`) 1.0)
      (if (not (`self.IsAttacking`))
        (`self.LaunchCharacter` (* _returnvalue 2000.0))
        (else
          (`self.LaunchCharacter` (* _returnvalue 8000.0))))
      (`self.PlayAnimMontage` "/Game/BLADE/montage/BLADE_DASH_Montage.BLADE_DASH_Montage")
      (set `self.DashCoolDown` 0.0)
      (if (< (`self.DashCoolDown`) 1.0) :!label _label
        (set `self.DashCoolDown` (+ (`self.DashCoolDown`) 0.2))
        (`KismetSystemLibrary.Delay` 0.6)
        (goto _label)))))

(event `InputAxis|ForwardBackward`
  (params (AxisValue :type "Float (single-precision)"))
  (if (`self.ismove`)
    (if (not (`self.IsAttacking`))
      (`self.AddMovementInput` (`KismetMathLibrary.GetForwardVector` (`KismetMathLibrary.MakeRotator` 0.0 0.0 (.yaw (`self.GetControlRotation`)))) AxisValue))))

(event `Key|LeftMouseButton`
  (params (Key :type "Key Structure"))
  (:`Pressed`
    (if (`self.IsAttacking`)
      (set `self.Is Go Next Combo` true)
      (else
        (set `self.IsAttacking` true)
        (`SceneComponent.SetHiddenInGame` (`self.Slash`) false true)
        (`self.PlayAnimMontage` "/Game/BLADE/montage/blade_attack1_Montage.blade_attack1_Montage")
        (`self.UpdateRotByMoveKey` (`self.Is Press Right Key`))
        (set `self.Attack Count` (+ (`self.Attack Count`) 1))))))

(event `OnAnimEnd_Attack`
  (set `self.IsAttacking` false)
  (set `self.Is Go Next Combo` false)
  (set `self.Combo Count` 0))

(event `OnAnim_CheckNextCombo`
  (if (`self.Is Go Next Combo`)
    (set `self.Is Go Next Combo` false)
    (bind _output_get (set `self.Combo Count` (+ (`self.Combo Count`) 1)))
    (switch `int` _output_get
      (:`1`
        (`self.PlayAnimMontage` "/Game/BLADE/montage/blade_attack2_Montage.blade_attack2_Montage"))
      (:`2`
        (`self.PlayAnimMontage` "/Game/BLADE/montage/blade_attack3_Montage.blade_attack3_Montage")))
    (`self.UpdateRotByMoveKey` (`self.Is Press Right Key`))))

(event `Key|SpaceBar`
  (params (Key :type "Key Structure"))
  (:`Pressed`
    (if (`NavMovementComponent.IsFalling` (`self.CharacterMovement`))
      _
      (elif (not (`self.IsAttacking`))
        (`self.Jump`)
        (`self.PlayAnimMontage` "/Game/BLADE/montage/BLADE_JUMP_Montage.BLADE_JUMP_Montage"))))
  (:`Released`
    (`self.StopJumping`)))

(event `self.Capsule.OnComponentBeginOverlap`
  (params (OverlappedComponent :type "PrimitiveComponent Object Reference") (OtherActor :type "Actor Object Reference") (OtherComp :type "PrimitiveComponent Object Reference") (OtherBodyIndex :type Integer) (bFromSweep :type Boolean) (SweepResult :type "HitResult Structure (by ref)"))
  (if (`self.IsAttacking`)
    (if (!= OtherActor self)
      (if (!= (`|GetArrayItem` (`self.Tags`)) (`|GetArrayItem` (`Actor.Tags` OtherActor)))
        (if (== (`|GetArrayItem` (`ActorComponent.ComponentTags` OtherComp)) "Character")
          (`GameplayStatics.ApplyDamage` OtherActor (`self.Atk`) null self)
          (`NiagaraFunctionLibrary.SpawnSystemAtLocation` "/Game/Assets/VFX/Niagara/FX_sword_hit.FX_sword_hit")
          (`GameplayStatics.PlaySoundAtLocation` "/Game/Assets/Sound/Charactor_Blade/swordclash_1and2.swordclash_1and2" (0.0 0.0 0.0) (struct) 1.0 1.0 0.0 null null null null))))))

(event `self.OnLanded`
  (params (Hit :type "HitResult Structure (by ref)"))
  (`self.StopAnimMontage` "/Game/BLADE/montage/BLADE_JUMP_Montage.BLADE_JUMP_Montage")
  (set `self.jumpCount` (+ (`self.jumpCount`) 1)))

(event `OnCollStart_Attack`
  (`PrimitiveComponent.SetCollisionEnabled` (`self.Capsule`) "QueryAndPhysics"))

(event `OnCollEnd_Attack`
  (`PrimitiveComponent.SetCollisionEnabled` (`self.Capsule`) "NoCollision"))

(event `self.ReceiveAnyDamage`
  (params (Damage :type "Float (single-precision)") (DamageType :type "DamageType Object Reference") (InstigatedBy :type "Controller Object Reference") (DamageCauser :type "Actor Object Reference"))
  (bind _returnvalue (`GameplayStatics.GetActorOfClass` "/Game/HellDemonBoss/HellDemonBP.HellDemonBP_C"))
  (if (`/Game/HellDemonBoss/HellDemonBP.aiAttack` _returnvalue)
    _
    (elif (not (`self.isNodamage`))
      (bind _output_get (set `self.Hp` (- (`self.Hp`) Damage)))
      (`/Game/Blueprints/Widgets/GamePlayMainWidget.Update_HeroHPBar` (`/Game/Blueprints/SideScrollGameInstance.gwmg` (`self.SideScrollGameInsRef`)) (`self.Hp`) (`self.MaxHp`))
      (`self.ChangeDamageColor`)
      (if (<= _output_get 0.0)
        (if (`self.LifeOff`)
          (`KismetSystemLibrary.PrintString` "Hello")
          (set `self.IsDeath` true)
          (else
            (bind _output_get_2 (set `self.DeathCount` (+ (`self.DeathCount`) 1.0)))
            (if (>= _output_get_2 2.0)
              (set `self.IsDeath` true)
              (else
                (bind _returnvalue_2 (`GameplayStatics.GetActorOfClass` "/Game/AI/Aiblade.Aiblade_C"))
                (set `/Game/AI/Aiblade.isdeathai` true _returnvalue_2)
                (`self.PlayAnimMontage` "/Game/BLADE/montage/BLADE_DEATH_Montage.BLADE_DEATH_Montage")
                (set `self.ismove` false)
                (bind _returnvalue_3 (`GameplayStatics.GetActorOfClass` "/Game/HellDemonBoss/HellDemonBP.HellDemonBP_C"))
                (set `/Game/HellDemonBoss/HellDemonBP.isMove` false _returnvalue_3)
                (`self.부활`)
                (`KismetSystemLibrary.Delay` 2.0)
                (set `self.ismove` true)
                (set `/Game/HellDemonBoss/HellDemonBP.isMove` true _returnvalue_3)))))))))

(event `ChangeDamageColor`
  (`PrimitiveComponent.SetMaterial` (`self.Mesh`) 0 "/Game/Mesh/Paladin/Paladin_MAT_Inst.Paladin_MAT_Inst")
  (`KismetSystemLibrary.Delay` 0.2)
  (`PrimitiveComponent.SetMaterial` (`self.Mesh`) 0 null))

(event `Key|R`
  (params (Key :type "Key Structure"))
  (:`Pressed`
    (if (>= (`self.MaskCount`) 1.0)
      (if (> (`self.Mp`) 0.0)
        (set `self.isSkilling` true)
        (if (`self.isSkilling`)
          (if (`NavMovementComponent.IsFalling` (`self.CharacterMovement`))
            _
            (elif (not (`self.IsAttacking`))
              (`SceneComponent.SetHiddenInGame` (`self.Slash`) false true)
              (set `self.IsAttacking` true)
              (`self.PlayAnimMontage` "/Game/BLADE/Animation/blade_skill3_Montage.blade_skill3_Montage")
              (bind _output_get (set `self.Mp` (- (`self.Mp`) (`self.Skill2Mp`))))
              (`/Game/Blueprints/Widgets/GamePlayMainWidget.Update_MPBar` (`/Game/Blueprints/SideScrollGameInstance.gwmg` (`self.SideScrollGameInsRef`)) (`self.Mp`) (`self.MaxMp`))
              (`KismetSystemLibrary.Delay` 2.0)
              (set `self.IsAttacking` false))))
        (else
          (set `self.isSkilling` false)))
      (else
        (`KismetSystemLibrary.PrintString` "스킬2 유물 부족")))))

(event `Key|F`
  (params (Key :type "Key Structure"))
  (:`Pressed`
    (if (>= (`self.jarCount`) 1.0)
      (if (> (`self.Mp`) 0.0)
        (set `self.isSkilling` true)
        (if (`self.isSkilling`)
          (if (`NavMovementComponent.IsFalling` (`self.CharacterMovement`))
            _
            (elif (not (`self.IsAttacking`))
              (`SceneComponent.SetHiddenInGame` (`self.Slash`) false true)
              (set `self.IsAttacking` true)
              (`self.PlayAnimMontage` "/Game/BLADE/montage/blade_skill_Montage.blade_skill_Montage")
              (set `self.Mp` (- (`self.Mp`) (`self.SkillMp`)))
              (`/Game/Blueprints/Widgets/GamePlayMainWidget.Update_MPBar` (`/Game/Blueprints/SideScrollGameInstance.gwmg` (`self.SideScrollGameInsRef`)) (`self.Mp`) (`self.MaxMp`))
              (`KismetSystemLibrary.Delay` 0.8)
              (set `self.IsAttacking` false))))
        (else
          (set `self.isSkilling` false)))
      (else
        (`KismetSystemLibrary.PrintString` "스킬1 유물 부족")))))

(event `Key|G`
  (params (Key :type "Key Structure"))
  (:`Pressed`
    (set `self.isSussNorGuard` true)
    (if (`self.isguard`)
      (set `self.isNodamage` true)
      (set `self.ismove` false)
      (`self.PlayAnimMontage` "/Game/BLADE/montage/blade_block_Montage.blade_block_Montage")
      (set `self.isguard` false)
      (`KismetSystemLibrary.Delay` 1.0)
      (set `self.isNodamage` false)
      (set `self.ismove` true)
      (set `self.isgTimer` true)
      (set `self.isSussNorGuard` false))))

(event `self.CapsuleSkill.OnComponentBeginOverlap`
  (params (OverlappedComponent :type "PrimitiveComponent Object Reference") (OtherActor :type "Actor Object Reference") (OtherComp :type "PrimitiveComponent Object Reference") (OtherBodyIndex :type Integer) (bFromSweep :type Boolean) (SweepResult :type "HitResult Structure (by ref)"))
  (if (!= OtherActor self)
    (if (!= (`|GetArrayItem` (`self.Tags`)) (`|GetArrayItem` (`Actor.Tags` OtherActor)))
      (if (== (`|GetArrayItem` (`ActorComponent.ComponentTags` OtherComp)) "Character")
        (`GameplayStatics.ApplyDamage` OtherActor (`self.skill Damage`) null self)
        (`NiagaraFunctionLibrary.SpawnSystemAtLocation` "/Game/Assets/VFX/Niagara/FX_sword_hit.FX_sword_hit")
        (`GameplayStatics.PlaySoundAtLocation` "/Game/Assets/Sound/Charactor_Blade/swordclash_1and2.swordclash_1and2" (0.0 0.0 0.0) (struct) 1.0 1.0 0.0 null null null null)))))

(event `guardTimer`
  (set `self.ismove` true)
  (`KismetSystemLibrary.Delay` 0.5)
  (bind _output_get (set `self.GuardCool` (+ (`self.GuardCool`) 1.0)))
  (`KismetSystemLibrary.PrintString` (`KismetStringLibrary.Conv_DoubleToString` _output_get))
  (if (>= (`self.GuardCool`) 5.0)
    (set `self.GuardCool` 0.0)
    (set `self.isguard` true)
    (set `self.isgTimer` false)))

(event `OnColStart_Skill1Attack`
  (`PrimitiveComponent.SetCollisionEnabled` (`self.CapsuleSkill`) "QueryAndPhysics"))

(event `OnColEnd_Skill1Attack`
  (`PrimitiveComponent.SetCollisionEnabled` (`self.CapsuleSkill`) "NoCollision"))

(event `InputAxis|Turn`
  (params (AxisValue :type "Float (single-precision)"))
  (`self.AddControllerYawInput` AxisValue))

(event `InputAxis|LookUp`
  (params (AxisValue :type "Float (single-precision)"))
  (`self.AddControllerPitchInput` AxisValue))

(event `OnColStart_Skill2Attack`
  (`PrimitiveComponent.SetCollisionEnabled` (`self.CapsuleSkill2`) "QueryAndPhysics"))

(event `OnColEnd_Skill2Attack`
  (`PrimitiveComponent.SetCollisionEnabled` (`self.CapsuleSkill2`) "NoCollision"))

(event `self.CapsuleSkill2.OnComponentBeginOverlap`
  (params (OverlappedComponent :type "PrimitiveComponent Object Reference") (OtherActor :type "Actor Object Reference") (OtherComp :type "PrimitiveComponent Object Reference") (OtherBodyIndex :type Integer) (bFromSweep :type Boolean) (SweepResult :type "HitResult Structure (by ref)"))
  (if (!= OtherActor self)
    (if (!= (`|GetArrayItem` (`self.Tags`)) (`|GetArrayItem` (`Actor.Tags` OtherActor)))
      (if (== (`|GetArrayItem` (`ActorComponent.ComponentTags` OtherComp)) "Character")
        (`GameplayStatics.ApplyDamage` OtherActor (`self.skill Damage`) null self)
        (`NiagaraFunctionLibrary.SpawnSystemAtLocation` "/Game/Assets/VFX/Niagara/FX_sword_hit.FX_sword_hit")
        (`GameplayStatics.PlaySoundAtLocation` "/Game/Assets/Sound/Charactor_Blade/swordclash_1and2.swordclash_1and2" (0.0 0.0 0.0) (struct) 1.0 1.0 0.0 null null null null)))))

(fn `UpdateRotByMoveKey`
  (params (IsPressRightKey :type Boolean)))

(fn `UserConstructionScript`)