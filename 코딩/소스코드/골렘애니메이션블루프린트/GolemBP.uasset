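; Golem boss character for a side-scroller that chases and attacks the Paladin player, showing a boss HP bar.
; Tick runs an enum state machine on Y-axis distance to the player: idle, follow, attack.
; StartAttack plays a basic montage, or a skill montage when a self-looping timer allows.
; Collision events toggle sphere and capsule hitboxes that apply tag-filtered damage; taking damage flashes the material, and death destroys the actor.
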(event `self.ReceiveBeginPlay`
  (bind _asside_scroll_game_instance (cast `/Game/Blueprints/SideScrollGameInstance` (`GameplayStatics.GetGameInstance`)))
  (set `self.SideScrollGameRef` _asside_scroll_game_instance))

(event `SkillTimeLoop`
  (`KismetSystemLibrary.Delay` 1.0)
  (set `self.SkillTime` (+ (`self.SkillTime`) 1.0))
  (`self.SkillTimeLoop`))

(event `self.ReceiveTick`
  (params (DeltaSeconds :type "Float (single-precision)"))
  (`self.SaveDisAndDir`)
  (if (`self.IsDeathPlayerChar`)
    (set `self.CurState` "NewEnumerator3"))
  (switch `/Game/Enums/MonsterState` (`self.CurState`)
    (:`NewEnumerator0`
      (if (<= (`self.DistancePlayerChar`) 500.0)
        (`/Game/Blueprints/SideScrollGameInstance.ShowBossUI` (`self.SideScrollGameRef`) true (`self.BossTexture`))
        (set `self.CurState` "NewEnumerator1")
        (`self.SkillTimeLoop`)))
    (:`NewEnumerator1`
      (if (<= (`self.DistancePlayerChar`) 130.0)
        (`self.StartAttack`)
        (else
          (`self.AddMovementInput` (`self.DirToPlayerChar`)))))
    (:`NewEnumerator2`
      (if (`self.IsAttacking`)
        _
        (elif (> (`self.DistancePlayerChar`) 150.0)
          (set `self.CurState` "NewEnumerator1"))))))

(event `OnAnimEnd_Attack`
  (`PrimitiveComponent.SetMaterial` (`self.Mesh`) 0 "/Game/DemoMesh/golem_Material__2.golem_Material__2")
  (set `self.IsAttacking` false)
  (if (`self.IsDeathPlayerChar`)
    (set `self.CurState` "NewEnumerator3")
    (elif (> (`self.DistancePlayerChar`) 180.0)
      (set `self.CurState` "NewEnumerator1")
      (else
        (`self.StartAttack`)))))

(event `StartAttack`
  (set `self.IsAttacking` true)
  (if (>= (`self.SkillTime`) 5.0)
    (set `self.CurState` "NewEnumerator5")
    (`self.K2_SetActorRotation` (`KismetMathLibrary.Conv_VectorToRotator` (`self.DirToPlayerChar`)))
    (set `self.SkillTime` 0.0)
    (`self.PlayAnimMontage` "/Game/DemoMesh/Montage/golem_attack2_montage.golem_attack2_montage" 1.0 "Start")
    (`KismetSystemLibrary.Delay` 10.0)
    (else
      (set `self.CurState` "NewEnumerator2")
      (`self.K2_SetActorRotation` (`KismetMathLibrary.Conv_VectorToRotator` (`self.DirToPlayerChar`)))
      (`self.PlayAnimMontage` "/Game/DemoMesh/Montage/golem_attack1_montage.golem_attack1_montage"))))

(event `SaveDisAndDir`
  (bind _returnvalue (`GameplayStatics.GetPlayerCharacter` 0))
  (bind _returnvalue_2 (`KismetMathLibrary.MakeVector` 0.0 (.y (- (`self.K2_GetActorLocation` _returnvalue) (`self.K2_GetActorLocation`)))))
  (bind _aspaladin_hero_bp (cast `/Game/Blueprints/PaladinHeroBP` _returnvalue))
  (set `self.IsDeathPlayerChar` (`/Game/Blueprints/PaladinHeroBP.IsDeath` _aspaladin_hero_bp))
  (set `self.DistancePlayerChar` (`KismetMathLibrary.VSize` _returnvalue_2))
  (set `self.DirToPlayerChar` (`KismetMathLibrary.Normal` _returnvalue_2)))

(event `self.ReceiveAnyDamage`
  (params (Damage :type "Float (single-precision)") (DamageType :type "DamageType Object Reference") (InstigatedBy :type "Controller Object Reference") (DamageCauser :type "Actor Object Reference"))
  (bind _output_get (set `self.Hp` (- (`self.Hp`) Damage)))
  (`/Game/Blueprints/Widgets/GamePlayMain.Update_BossHPBar` (`/Game/Blueprints/SideScrollGameInstance.GamePlayMainWidgetRef` (`self.SideScrollGameRef`)) (`self.Hp`) (`self.MaxHp`))
  (`self.ChangeDamageColor`)
  (if (<= _output_get 0.0)
    (`self.PlayAnimMontage` "/Game/Mesh/Boss1/AnimMontage/mutant_dying_Montage.mutant_dying_Montage")
    (set `self.CurState` "NewEnumerator4")
    (`PrimitiveComponent.SetCollisionEnabled` (`self.CapsuleComponent`) "NoCollision")
    (`PrimitiveComponent.SetCollisionEnabled` (`self.Capsule`) "NoCollision")
    (`PrimitiveComponent.SetCollisionEnabled` (`self.Sphere`) "NoCollision")
    (`KismetSystemLibrary.Delay` 0.5)
    (`self.K2_DestroyActor`)))

(event `ChangeDamageColor`
  (`GameplayStatics.SpawnEmitterAttached` "/Game/InfinityBladeEffects/Effects/FX_Mobile/Fire/combat/P_FireBall_Powerup.P_FireBall_Powerup" (`self.CapsuleComponent`))
  (`PrimitiveComponent.SetMaterial` (`self.Mesh`) 0 "/Game/Mesh/Boss1/mutant_M_Inst.mutant_M_Inst")
  (`KismetSystemLibrary.Delay` 0.2)
  (`PrimitiveComponent.SetMaterial` (`self.Mesh`) 0 "/Game/Mesh/Boss1/mutant_M.mutant_M"))

(event `self.Capsule.OnComponentBeginOverlap`
  (params (OverlappedComponent :type "PrimitiveComponent Object Reference") (OtherActor :type "Actor Object Reference") (OtherComp :type "PrimitiveComponent Object Reference") (OtherBodyIndex :type Integer) (bFromSweep :type Boolean) (SweepResult :type "HitResult Structure (by ref)"))
  (if (!= OtherActor self)
    (if (!= (`|GetArrayItem` (`self.Tags`)) (`|GetArrayItem` (`Actor.Tags` OtherActor)))
      (if (== (`|GetArrayItem` (`ActorComponent.ComponentTags` OtherComp)) "Character")
        (`GameplayStatics.ApplyDamage` OtherActor (`self.Skill1Atk`) null self)))))

(event `self.Sphere.OnComponentBeginOverlap`
  (params (OverlappedComponent :type "PrimitiveComponent Object Reference") (OtherActor :type "Actor Object Reference") (OtherComp :type "PrimitiveComponent Object Reference") (OtherBodyIndex :type Integer) (bFromSweep :type Boolean) (SweepResult :type "HitResult Structure (by ref)"))
  (if (!= OtherActor self)
    (if (!= (`|GetArrayItem` (`self.Tags`)) (`|GetArrayItem` (`Actor.Tags` OtherActor)))
      (if (== (`|GetArrayItem` (`ActorComponent.ComponentTags` OtherComp)) "Character")
        (`GameplayStatics.ApplyDamage` OtherActor (`self.Atk`) null self)))))

(event `OnColStart_Attack`
  (`PrimitiveComponent.SetCollisionEnabled` (`self.Sphere`) "QueryAndPhysics"))

(event `OnColEnd_Attack`
  (`PrimitiveComponent.SetCollisionEnabled` (`self.Sphere`) "NoCollision"))

(event `OnColStart_Skill1Attack`
  (`PrimitiveComponent.SetCollisionEnabled` (`self.Capsule`) "QueryAndPhysics"))

(event `OnColEnd_Skill1Attack`
  (`PrimitiveComponent.SetCollisionEnabled` (`self.Capsule`) "NoCollision"))

(fn `UserConstructionScript`)