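; Ghost enemy that locks onto the first BladeBP or CShooterBP player found nearest within range, then chases and melees it.
; Tick refreshes distance and direction, driving an idle, follow and attack state machine with montages and tag-filtered hit capsules.
; Damage shows a number and material flash; death plays Niagara FX and increments player 0's BladeBP KillCount, spawning a pendant from six kills.
; The HP bar spawn is unwired, though damage updates it.
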(event `self.ReceiveBeginPlay`)

(event `self.ReceiveTick`
  (params (DeltaSeconds :type "Float (single-precision)"))
  (`self.SaveDisAndDir`)
  (if (or (`self.IsDeathPlayerChar`) (`self.IsStageClear`))
    (set `self.CurState` "NewEnumerator3"))
  (switch `/Game/Enums/MonsterState` (`self.CurState`)
    (:`NewEnumerator0`
      (if (<= (`self.DistancePlayerChar`) 500.0)
        (set `self.CurState` "NewEnumerator1")))
    (:`NewEnumerator1`
      (if (<= (`self.DistancePlayerChar`) 160.0)
        (set `self.CurState` "NewEnumerator2")
        (`self.PlayAnimMontage` "/Game/Monster/ghost/GhostAttackMontage.GhostAttackMontage")
        (set `self.IsAttacking` true)
        (else
          (`self.AddMovementInput` (`self.DirToPlayerChar`)))))
    (:`NewEnumerator2`
      (if (`self.IsAttacking`)
        _
        (elif (> (`self.DistancePlayerChar`) 180.0)
          (set `self.CurState` "NewEnumerator1"))))))

(event `OnAnimEnd_Attack`
  (set `self.IsAttacking` false)
  (if (or (`self.IsDeathPlayerChar`) (`self.IsStageClear`))
    (set `self.CurState` "NewEnumerator3")
    (elif (> (`self.DistancePlayerChar`) 180.0)
      (set `self.CurState` "NewEnumerator1")
      (else
        (`self.K2_SetActorRotation` (`KismetMathLibrary.Conv_VectorToRotator` (`self.DirToPlayerChar`)))
        (`self.PlayAnimMontage` "/Game/Monster/ghost/GhostAttackMontage.GhostAttackMontage")
        (set `self.IsAttacking` true)))))

(event `SaveDisAndDir`
  (switch `int` (`self.monsterTarget`)
    (:`0`
      (`self.distance`))
    (:`1`
      (bind _outactors (`GameplayStatics.GetAllActorsOfClass` "/Game/BLADE/BladeBP.BladeBP_C"))
      (bind _returnvalue (`KismetMathLibrary.MakeVector` (.x (- (`self.K2_GetActorLocation` (`|GetArrayItem` _outactors)) (`self.K2_GetActorLocation`))) (.y (- (`self.K2_GetActorLocation` (`|GetArrayItem` _outactors)) (`self.K2_GetActorLocation`))) (.z (- (`self.K2_GetActorLocation` (`|GetArrayItem` _outactors)) (`self.K2_GetActorLocation`)))))
      (set `self.DistancePlayerChar` (`KismetMathLibrary.VSize` _returnvalue))
      (set `self.DirToPlayerChar` (`KismetMathLibrary.Normal` _returnvalue)))
    (:`2`
      (bind _outactors_2 (`GameplayStatics.GetAllActorsOfClass` "/Game/CANNONSHOOTER/CShooterBP.CShooterBP_C"))
      (bind _returnvalue_2 (`KismetMathLibrary.MakeVector` (.x (- (`self.K2_GetActorLocation` (`|GetArrayItem` _outactors_2)) (`self.K2_GetActorLocation`))) (.y (- (`self.K2_GetActorLocation` (`|GetArrayItem` _outactors_2)) (`self.K2_GetActorLocation`))) (.z (- (`self.K2_GetActorLocation` (`|GetArrayItem` _outactors_2)) (`self.K2_GetActorLocation`)))))
      (set `self.DistancePlayerChar` (`KismetMathLibrary.VSize` _returnvalue_2))
      (set `self.DirToPlayerChar` (`KismetMathLibrary.Normal` _returnvalue_2)))))

(event `distance`
  (bind _outactors (`GameplayStatics.GetAllActorsOfClass` "/Game/BLADE/BladeBP.BladeBP_C"))
  (bind _outactors_2 (`GameplayStatics.GetAllActorsOfClass` "/Game/CANNONSHOOTER/CShooterBP.CShooterBP_C"))
  (bind _returnvalue (`self.GetDistanceTo` (`|GetArrayItem` _outactors_2) self))
  (bind _returnvalue_2 (`self.GetDistanceTo` (`|GetArrayItem` _outactors) self))
  (if (>= (- _returnvalue _returnvalue_2) 0.0)
    (if (<= _returnvalue_2 500.0)
      (set `self.monsterTarget` 1))
    (elif (<= _returnvalue 500.0)
      (set `self.monsterTarget` 2))))

(event `self.ReceiveAnyDamage`
  (params (Damage :type "Float (single-precision)") (DamageType :type "DamageType Object Reference") (InstigatedBy :type "Controller Object Reference") (DamageCauser :type "Actor Object Reference"))
  (set `self.Damage` Damage)
  (bind _output_get (set `self.Hp` (- (`self.Hp`) Damage)))
  (`/Game/BLUEPRINT/HpBarBPMonster.UpdateMaxHpBar` (`self.HpBarActor`) (`self.Hp`) (`self.MaxHp`))
  (`self.ChangeDamageColor`)
  (if (<= _output_get 0.0)
    (set `self.deathcount` (+ (`self.deathcount`) 1.0))
    (set `self.CurState` "NewEnumerator4")
    (`self.K2_DestroyActor` (`self.HpBarActor`))
    (`KismetSystemLibrary.Delay` 0.1)
    (`NiagaraFunctionLibrary.SpawnSystemAtLocation` "/Game/Assets/VFX/Niagara/New_Effects/FX_GhostKill.FX_GhostKill" (`SceneComponent.K2_GetComponentLocation` (`self.eyebeam`)))
    (`self.K2_DestroyActor`)
    (bind _asblade_bp (cast `/Game/BLADE/BladeBP` (`GameplayStatics.GetPlayerCharacter` 0)))
    (bind _output_get_2 (set `/Game/BLADE/BladeBP.killCount` (+ (`/Game/BLADE/BladeBP.killCount` _asblade_bp) 1.0) _asblade_bp))
    (if (>= _output_get_2 6.0)
      (`|SpawnActorFromClass` "/Game/BLUEPRINT/BP_pendent.BP_pendent_C" (`self.GetTransform`) "Undefined" "OverrideRootScale" null null))))

(event `ChangeDamageColor`
  (bind _returnvalue (`|SpawnActorFromClass` "/Game/BLADE/BP_TestDamage.BP_TestDamage_C" (`KismetMathLibrary.MakeTransform` (+ (`SceneComponent.K2_GetComponentLocation` (`self.damageDummy`)) (0.0 0.0 60.0))) "Undefined" "OverrideRootScale" null null))
  (`/Game/BLADE/BP_TestDamage.Set DamegeText` _returnvalue (`self.Damage`))
  (`KismetSystemLibrary.Delay` 0.2)
  (`self.K2_DestroyActor` _returnvalue)
  (`GameplayStatics.SpawnEmitterAttached` null (`self.CapsuleComponent`))
  (`PrimitiveComponent.SetMaterial` (`self.Mesh`) 0 "/Game/Assets/Material/MM_warning.MM_warning")
  (`KismetSystemLibrary.Delay` 0.2)
  (`PrimitiveComponent.SetMaterial` (`self.Mesh`) 0 "/Game/Assets/Material/MM_Ghost.MM_Ghost"))

(event `self.CapsuleRight.OnComponentBeginOverlap`
  (params (OverlappedComponent :type "PrimitiveComponent Object Reference") (OtherActor :type "Actor Object Reference") (OtherComp :type "PrimitiveComponent Object Reference") (OtherBodyIndex :type Integer) (bFromSweep :type Boolean) (SweepResult :type "HitResult Structure (by ref)"))
  (if (!= OtherActor self)
    (if (!= (`|GetArrayItem` (`self.Tags`)) (`|GetArrayItem` (`Actor.Tags` OtherActor)))
      (if (== (`|GetArrayItem` (`ActorComponent.ComponentTags` OtherComp)) "ghCharacter")
        (`GameplayStatics.ApplyDamage` OtherActor (`self.Atk`) null self)))))

(event `self.CapsuleLeft.OnComponentBeginOverlap`
  (params (OverlappedComponent :type "PrimitiveComponent Object Reference") (OtherActor :type "Actor Object Reference") (OtherComp :type "PrimitiveComponent Object Reference") (OtherBodyIndex :type Integer) (bFromSweep :type Boolean) (SweepResult :type "HitResult Structure (by ref)"))
  (if (!= OtherActor self)
    (if (!= (`|GetArrayItem` (`self.Tags`)) (`|GetArrayItem` (`Actor.Tags` OtherActor)))
      (if (== (`|GetArrayItem` (`ActorComponent.ComponentTags` OtherComp)) "ghCharacter")
        (`GameplayStatics.ApplyDamage` OtherActor (`self.Atk`) null self)))))

(event `OnColStart_Attack`
  (`PrimitiveComponent.SetCollisionEnabled` (`self.CapsuleRight`) "QueryAndPhysics"))

(event `OnColEnd_Attack`
  (`PrimitiveComponent.SetCollisionEnabled` (`self.CapsuleRight`) "NoCollision"))

(fn `UserConstructionScript`)