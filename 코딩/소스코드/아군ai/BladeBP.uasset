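; BladeBP is the playable sword character, with movement, jump, cooldown dash, a three-hit melee combo and an MP-costing skill.
; Animation-driven events advance the combo and toggle attack and skill capsules, whose overlaps damage characters with a different tag.
; Damage, healing and a save event's stat refill update HP/MP bars through the game instance.
; Death prints item tallies, shows StageFail, disables input and spawns a Bladeai in its place.
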(event `save`
  (set `self.Hp` 200.0)
  (`/Game/Blueprints/Widgets/GamePlayMainWidget.Update_HeroHPBar` (`/Game/Blueprints/SideScrollGameInstance.gwmg` (`self.SideScrollGameInsRef`)) (`self.Hp`) (`self.MaxHp`))
  (set `self.Mp` 100.0)
  (`/Game/Blueprints/Widgets/GamePlayMainWidget.Update_MPBar` (`/Game/Blueprints/SideScrollGameInstance.gwmg` (`self.SideScrollGameInsRef`)) (`self.Mp`) (`self.MaxMp`)))

(event `self.ReceiveBeginPlay`
  (bind _asside_scroll_game_instance (cast `/Game/Blueprints/SideScrollGameInstance` (`GameplayStatics.GetGameInstance`)))
  (set `self.SideScrollGameInsRef` _asside_scroll_game_instance)
  (set `self.isSave` false)
  (set `self.isPendent` false))

(event `self.ReceiveTick`
  (params (DeltaSeconds :type "Float (single-precision)"))
  (bind _returnvalue (`GameplayStatics.GetPlayerController` 0))
  (if (`self.IsDeath`)
    (`/Engine/EditorBlueprintResources/StandardMacros.DoOnce` false
      (:`Completed`
        (`KismetSystemLibrary.PrintText` (`|FormatText` "score : {n}" (`self.GemCount`)))
        (`KismetSystemLibrary.PrintText` (`|FormatText` "Mask : {n}" (`self.MaskCount`)))
        (`KismetSystemLibrary.PrintText` (`|FormatText` "jar : {n}" (`self.jarCount`)))
        (`KismetSystemLibrary.PrintText` (`|FormatText` "grail : {n}" (`self.grailCount`)))
        (`KismetSystemLibrary.PrintText` (`|FormatText` "공격력 상승량 : {n}" (+ (* (`self.jarCount`) 10.0) (* (`self.grailCount`) 10.0))))
        (`KismetSystemLibrary.PrintText` (`|FormatText` "방어력 상승량 : {n}" (* (`self.MaskCount`) 10.0)))
        (`self.PlayAnimMontage` "/Game/BLADE/montage/BLADE_DEATH_Montage.BLADE_DEATH_Montage")
        (bind _returnvalue_2 (`|CreateWidget` "/Game/Blueprints/Widgets/StageFail.StageFail_C" _returnvalue))
        (`UserWidget.AddToViewport` _returnvalue_2 0)
        (set `PlayerController.bShowMouseCursor` true _returnvalue)
        (`self.DisableInput` (`GameplayStatics.GetPlayerCharacter` 0) (`GameplayStatics.GetPlayerController` 0))
        (`KismetSystemLibrary.Delay` 2.0)
        (`ActorComponent.K2_DestroyComponent` (`self.Mesh`))
        (`|SpawnActorFromClass` "/Game/AI/임시/bladeai.bladeai_C" (`self.GetTransform`) "Undefined" "OverrideRootScale" null null)))))

(event `heal`
  (if (`self.is heal`)
    (set `self.Hp` (+ (`self.Hp`) 10.0))
    (`/Game/Blueprints/Widgets/GamePlayMainWidget.Update_HeroHPBar` (`/Game/Blueprints/SideScrollGameInstance.gwmg` (`self.SideScrollGameInsRef`)) (`self.Hp`) (`self.MaxHp`))
    (set `self.is heal` false)))

(event `MpHeal`
  (if (`self.ismpHeal`)
    (set `self.Mp` (+ (`self.Mp`) 10.0))
    (`/Game/Blueprints/Widgets/GamePlayMainWidget.Update_MPBar` (`/Game/Blueprints/SideScrollGameInstance.gwmg` (`self.SideScrollGameInsRef`)) (`self.Mp`) (`self.MaxMp`))
    (set `self.ismpHeal` false)))

(event `Key|LeftShift`
  (params (Key :type "Key Structure"))
  (:`Pressed`
    (if (>= (`self.DashCoolDown`) 1.0)
      (if (not (`self.IsAttacking`))
        (`self.LaunchCharacter` (* (`self.GetActorForwardVector`) 2000.0))
        (`self.PlayAnimMontage` "/Game/BLADE/montage/BLADE_DASH_Montage.BLADE_DASH_Montage")
        (set `self.DashCoolDown` 0.0)
        (if (< (`self.DashCoolDown`) 1.0) :!label _label
          (set `self.DashCoolDown` (+ (`self.DashCoolDown`) 0.2))
          (`KismetSystemLibrary.Delay` 0.6)
          (goto _label))))))

(event `InputAxis|LeftRight`
  (params (AxisValue :type "Float (single-precision)"))
  (if (not (`self.IsAttacking`))
    (`SceneComponent.SetHiddenInGame` (`self.Slash`) true true)
    (`self.AddMovementInput` (`KismetMathLibrary.GetRightVector` (`KismetMathLibrary.MakeRotator` 0.0 0.0 (.yaw (`self.GetControlRotation`)))) AxisValue)))

(event `InputAxis|ForwardBackward`
  (params (AxisValue :type "Float (single-precision)"))
  (if (not (`self.IsAttacking`))
    (`self.AddMovementInput` (`KismetMathLibrary.GetForwardVector` (`KismetMathLibrary.MakeRotator` 0.0 0.0 (.yaw (`self.GetControlRotation`)))) AxisValue)))

(event `Key|LeftMouseButton`
  (params (Key :type "Key Structure"))
  (:`Pressed`
    (if (`self.IsAttacking`)
      (set `self.Is Go Next Combo` true)
      (else
        (set `self.IsAttacking` true)
        (`SceneComponent.SetHiddenInGame` (`self.Slash`) false true)
        (`self.PlayAnimMontage` "/Game/BLADE/montage/blade_attack1_Montage.blade_attack1_Montage")
        (`self.UpdateRotByMoveKey` (`self.Is Press Right Key`))
        (set `self.Attack Count` (+ (`self.Attack Count`) 1))))))

(event `OnAnimEnd_Attack`
  (set `self.IsAttacking` false)
  (set `self.Is Go Next Combo` false)
  (set `self.Combo Count` 0))

(event `OnAnim_CheckNextCombo`
  (if (`self.Is Go Next Combo`)
    (set `self.Is Go Next Combo` false)
    (bind _output_get (set `self.Combo Count` (+ (`self.Combo Count`) 1)))
    (switch `int` _output_get
      (:`1`
        (`self.PlayAnimMontage` "/Game/BLADE/montage/blade_attack2_Montage.blade_attack2_Montage"))
      (:`2`
        (`self.PlayAnimMontage` "/Game/BLADE/montage/blade_attack3_Montage.blade_attack3_Montage")))
    (`self.UpdateRotByMoveKey` (`self.Is Press Right Key`))))

(event `Key|SpaceBar`
  (params (Key :type "Key Structure"))
  (:`Pressed`
    (if (`NavMovementComponent.IsFalling` (`self.CharacterMovement`))
      _
      (elif (not (`self.IsAttacking`))
        (`self.Jump`)
        (`self.PlayAnimMontage` "/Game/BLADE/montage/BLADE_JUMP_Montage.BLADE_JUMP_Montage"))))
  (:`Released`
    (`self.StopJumping`)))

(event `self.Capsule.OnComponentBeginOverlap`
  (params (OverlappedComponent :type "PrimitiveComponent Object Reference") (OtherActor :type "Actor Object Reference") (OtherComp :type "PrimitiveComponent Object Reference") (OtherBodyIndex :type Integer) (bFromSweep :type Boolean) (SweepResult :type "HitResult Structure (by ref)"))
  (if (`self.IsAttacking`)
    (if (!= OtherActor self)
      (if (!= (`|GetArrayItem` (`self.Tags`)) (`|GetArrayItem` (`Actor.Tags` OtherActor)))
        (if (== (`|GetArrayItem` (`ActorComponent.ComponentTags` OtherComp)) "Character")
          (`GameplayStatics.ApplyDamage` OtherActor (`KismetMathLibrary.Conv_IntToDouble` (`KismetMathLibrary.RandomIntegerInRange` 32 40)) null self)
          (`NiagaraFunctionLibrary.SpawnSystemAtLocation` "/Game/Assets/VFX/Niagara/FX_sword_hit.FX_sword_hit")
          (`GameplayStatics.PlaySoundAtLocation` "/Game/Assets/Sound/Charactor_Blade/swordclash_1and2.swordclash_1and2" (0.0 0.0 0.0) (struct) 1.0 1.0 0.0 null null null null))))))

(event `self.OnLanded`
  (params (Hit :type "HitResult Structure (by ref)"))
  (`self.StopAnimMontage` "/Game/BLADE/montage/BLADE_JUMP_Montage.BLADE_JUMP_Montage")
  (set `self.jumpCount` (+ (`self.jumpCount`) 1)))

(event `OnCollStart_Attack`
  (`PrimitiveComponent.SetCollisionEnabled` (`self.Capsule`) "QueryAndPhysics"))

(event `OnCollEnd_Attack`
  (`PrimitiveComponent.SetCollisionEnabled` (`self.Capsule`) "NoCollision"))

(event `self.ReceiveAnyDamage`
  (params (Damage :type "Float (single-precision)") (DamageType :type "DamageType Object Reference") (InstigatedBy :type "Controller Object Reference") (DamageCauser :type "Actor Object Reference"))
  (bind _output_get (set `self.Hp` (- (`self.Hp`) Damage)))
  (`/Game/Blueprints/Widgets/GamePlayMainWidget.Update_HeroHPBar` (`/Game/Blueprints/SideScrollGameInstance.gwmg` (`self.SideScrollGameInsRef`)) (`self.Hp`) (`self.MaxHp`))
  (`self.ChangeDamageColor`)
  (if (<= _output_get 0.0)
    (`self.PlayAnimMontage` "/Game/BLADE/montage/BLADE_DEATH_Montage.BLADE_DEATH_Montage")
    (set `self.IsDeath` true)))

(event `InputAxis|Turn`
  (params (AxisValue :type "Float (single-precision)"))
  (`self.AddControllerYawInput` AxisValue))

(event `ChangeDamageColor`
  (`PrimitiveComponent.SetMaterial` (`self.Mesh`) 0 "/Game/Mesh/Paladin/Paladin_MAT_Inst.Paladin_MAT_Inst")
  (`KismetSystemLibrary.Delay` 0.2)
  (`PrimitiveComponent.SetMaterial` (`self.Mesh`) 0 "/Game/InfinityBladeIceLands/Maps/LevelContent/Architecture/M_1Meter_01.M_1Meter_01"))

(event `InputAxis|LookUp`
  (params (AxisValue :type "Float (single-precision)"))
  (`self.AddControllerPitchInput` AxisValue))

(event `Key|F`
  (params (Key :type "Key Structure"))
  (:`Pressed`
    (if (> (`self.Mp`) 0.0)
      (set `self.isSkilling` true)
      (if (`self.isSkilling`)
        (if (`NavMovementComponent.IsFalling` (`self.CharacterMovement`))
          _
          (elif (not (`self.IsAttacking`))
            (`SceneComponent.SetHiddenInGame` (`self.Slash`) false true)
            (set `self.IsAttacking` true)
            (`self.PlayAnimMontage` "/Game/BLADE/montage/blade_skill_Montage.blade_skill_Montage")
            (bind _output_get (set `self.Mp` (- (`self.Mp`) (`self.SkillMp`))))
            (`/Game/Blueprints/Widgets/GamePlayMainWidget.Update_MPBar` (`/Game/Blueprints/SideScrollGameInstance.gwmg` (`self.SideScrollGameInsRef`)) (`self.Mp`) (`self.MaxMp`))
            (`KismetSystemLibrary.Delay` 0.8)
            (set `self.IsAttacking` false))))
      (else
        (set `self.isSkilling` false)))))

(event `self.CapsuleSkill.OnComponentBeginOverlap`
  (params (OverlappedComponent :type "PrimitiveComponent Object Reference") (OtherActor :type "Actor Object Reference") (OtherComp :type "PrimitiveComponent Object Reference") (OtherBodyIndex :type Integer) (bFromSweep :type Boolean) (SweepResult :type "HitResult Structure (by ref)"))
  (if (!= OtherActor self)
    (if (!= (`|GetArrayItem` (`self.Tags`)) (`|GetArrayItem` (`Actor.Tags` OtherActor)))
      (if (== (`|GetArrayItem` (`ActorComponent.ComponentTags` OtherComp)) "Character")
        (`GameplayStatics.ApplyDamage` OtherActor (`self.skill Damage`) null self)
        (`NiagaraFunctionLibrary.SpawnSystemAtLocation` "/Game/Assets/VFX/Niagara/FX_sword_hit.FX_sword_hit")
        (`GameplayStatics.PlaySoundAtLocation` "/Game/Assets/Sound/Charactor_Blade/swordclash_1and2.swordclash_1and2" (0.0 0.0 0.0) (struct) 1.0 1.0 0.0 null null null null)))))

(event `OnColStart_Skill1Attack`
  (`PrimitiveComponent.SetCollisionEnabled` (`self.CapsuleSkill`) "QueryAndPhysics"))

(event `OnColEnd_Skill1Attack`
  (`PrimitiveComponent.SetCollisionEnabled` (`self.CapsuleSkill`) "NoCollision"))

(fn `UpdateRotByMoveKey`
  (params (IsPressRightKey :type Boolean)))

(fn `UserConstructionScript`)