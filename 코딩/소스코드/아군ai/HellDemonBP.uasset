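; HellDemon final boss that chases and attacks the player or the Aiblade AI, switching target on a timer and showing its HP on the boss bar.
; Tick drives a state machine that picks a timed sweeping skill or a normal attack, with events toggling each attack's hit capsule.
; HP thresholds trigger one-time invulnerable montages, including an enrage that raises damage.
; Death plays effects and opens the final-stage clear widget.
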(event `행동시작`)

(event `chtargetcool`
  (`KismetSystemLibrary.Delay` 1.0)
  (set `self.Chartargetting` (+ (`self.Chartargetting`) 1.0))
  (if (>= (`self.Chartargetting`) 15.0)
    (set `self.Chartargetting` 0.0)
    (set `self.isaicool` true)
    (set `self.ischcool` false)))

(event `aitargetcool`
  (bind _returnvalue (`GameplayStatics.GetActorOfClass` "/Game/AI/Aiblade.Aiblade_C"))
  (if (not (`/Game/AI/Aiblade.isdeathai` _returnvalue))
    (`KismetSystemLibrary.Delay` 1.0)
    (set `self.Aitargetting` (+ (`self.Aitargetting`) 1.0))
    (if (>= (`self.Aitargetting`) 15.0)
      (set `self.Aitargetting` 0.0)
      (set `self.ischcool` true)
      (set `self.isaicool` false))))

(event `self.ReceiveBeginPlay`
  (set `self.isMove` true)
  (set `self.isAttack` false)
  (bind _asside_scroll_game_instance (cast `/Game/Blueprints/SideScrollGameInstance` (`GameplayStatics.GetGameInstance`)))
  (set `self.SideScrollGameRef` _asside_scroll_game_instance)
  (set `self.Hp` 300.0)
  (`/Game/Blueprints/Widgets/GamePlayMainWidget.Update_BossHPBar` (`/Game/Blueprints/SideScrollGameInstance.gwmg` (`self.SideScrollGameRef`)) (`self.Hp`) (`self.MaxHp`))
  (`/Engine/EditorBlueprintResources/StandardMacros.DoOnce` false
    (:`Completed`
      (set `self.isAttack` true)
      (set `self.DistancePlayerChar` 0.0))))

(event `SkillTimeLoop`
  (`KismetSystemLibrary.Delay` 1.0)
  (set `self.SkillTime` (+ (`self.SkillTime`) 1.0))
  (`self.SkillTimeLoop`))

(event `self.ReceiveTick`
  (params (DeltaSeconds :type "Float (single-precision)"))
  (bind _returnvalue (`GameplayStatics.GetPlayerController` 0))
  (bind _sidescrollgameref (`self.SideScrollGameRef`))
  (bind _bosstexture (`self.BossTexture`))
  (`|ExecutionSequence`
    (:`then_0`
      (if (not (`self.isRetarget`))
        (if (`self.ischcool`)
          (`self.chtargetcool`)
          (`self.SaveDisAndDir`)
          (else
            (`self.aitargetcool`)
            (`self.Aitarget`)))
        (if (`self.IsDeathPlayerChar`)
          (set `self.CurState` "NewEnumerator3"))
        (switch `/Game/Enums/MonsterState` (`self.CurState`)
          (:`NewEnumerator0`
            (if (<= (`self.DistancePlayerChar`) 10000.0)
              (`/Game/Blueprints/SideScrollGameInstance.ShowBossUI` _sidescrollgameref true _bosstexture)
              (set `self.CurState` "NewEnumerator1")
              (`self.SkillTimeLoop`)
              (else
                (`/Game/Blueprints/SideScrollGameInstance.ShowBossUI` _sidescrollgameref false _bosstexture)
                (set `self.CurState` "NewEnumerator0"))))
          (:`NewEnumerator1`
            (if (<= (`self.DistancePlayerChar`) 300.0)
              (`self.StartAttack`)
              (elif (not (> (`self.DistancePlayerChar`) 10000.0))
                (`self.AddMovementInput` (`self.DirToPlayerChar`)))))
          (:`NewEnumerator2`
            (if (`self.isAttack`)
              (if (`self.IsAttacking`)
                _
                (elif (> (`self.DistancePlayerChar`) 10000.0)
                  (set `self.CurState` "NewEnumerator1")))))
          (:`NewEnumerator4`
            (bind _returnvalue_2 (`|CreateWidget` "/Game/Blueprints/Widgets/FinalStageClear.FinalStageClear_C" _returnvalue))
            (`UserWidget.AddToViewport` _returnvalue_2 0)
            (set `PlayerController.bShowMouseCursor` true _returnvalue)
            (`self.DisableInput` (`GameplayStatics.GetPlayerCharacter` 0) (`GameplayStatics.GetPlayerController` 0))
            (`KismetSystemLibrary.Delay` 2.0)
            (`ActorComponent.K2_DestroyComponent` (`self.Mesh`))))))
    (:`then_1`
      (if (<= (`self.Hp`) 150.0)
        (`PrimitiveComponent.SetMaterial` (`self.Mesh`) 0 "/Game/Assets/Material/M_Lava_New.M_Lava_New")
        (`/Engine/EditorBlueprintResources/StandardMacros.DoOnce` false
          (:`Completed`
            (set `self.isMove` false)
            (set `self.isNoDamage` true)
            (`self.PlayAnimMontage` "/Game/HellDemonBoss/Montage/Boss_HellDemon_Roar_Montage.Boss_HellDemon_Roar_Montage")
            (`KismetSystemLibrary.Delay` 7.0)
            (set `self.isMove` true)
            (set `self.isNoDamage` false)
            (set `self.Atk` 20.0)
            (set `self.Skill1Atk` 40.0)
            (`self.StartAttack`)))))
    (:`then_2`
      (if (`self.isDamaged`)
        (set `self.Hp` (- (`self.Hp`) 3.0))
        (`/Game/Blueprints/Widgets/GamePlayMainWidget.Update_BossHPBar` (`/Game/Blueprints/SideScrollGameInstance.gwmg` (`self.SideScrollGameRef`)) (`self.Hp`) (`self.MaxHp`))
        (set `self.isDamaged` false)))
    (:`then_3`
      (if (<= (`self.Hp`) 220.0)
        (`/Engine/EditorBlueprintResources/StandardMacros.DoOnce` false
          (:`Completed`
            (set `self.isMove` false)
            (set `self.isNoDamage` true)
            (`self.PlayAnimMontage` "/Game/HellDemonBoss/Montage/Boss_HellDemon_Breath_Montage.Boss_HellDemon_Breath_Montage")
            (`KismetSystemLibrary.Delay` 3.0)
            (set `self.isMove` true)
            (set `self.isNoDamage` false)
            (`self.StartAttack`)))))
    (:`then_4`
      (if (<= (`self.Hp`) 80.0)
        (`/Engine/EditorBlueprintResources/StandardMacros.DoOnce` false
          (:`Completed`
            (set `self.isMove` false)
            (set `self.isNoDamage` true)
            (`self.PlayAnimMontage` "/Game/HellDemonBoss/Montage/Boss_HellDemon_JumpAttack_Montage.Boss_HellDemon_JumpAttack_Montage")
            (`KismetSystemLibrary.Delay` 4.0)
            (set `self.isMove` true)
            (set `self.isNoDamage` false)
            (`self.StartAttack`)))))))

(event `save`
  (`KismetSystemLibrary.PrintString` "보스제력세이브")
  (set `self.Hp` 100.0)
  (`/Game/Blueprints/Widgets/GamePlayMainWidget.Update_BossHPBar` (`/Game/Blueprints/SideScrollGameInstance.gwmg` (`self.SideScrollGameRef`)) (`self.Hp`) (`self.MaxHp`)))

(event `OnAnimEnd_Attack`
  (set `self.IsAttacking` false)
  (if (`self.IsDeathPlayerChar`)
    (set `self.CurState` "NewEnumerator3")
    (elif (> (`self.DistancePlayerChar`) 180.0)
      (set `self.CurState` "NewEnumerator1")
      (else
        (`self.StartAttack`)))))

(event `StartAttack`
  (if (`self.isMove`)
    (set `self.IsAttacking` true)
    (if (>= (`self.SkillTime`) 5.0)
      (set `self.isSkill` true)
      (set `self.isNormal` false)
      (set `self.CurState` "NewEnumerator5")
      (`self.K2_SetActorRotation` (`KismetMathLibrary.Conv_VectorToRotator` (`self.DirToPlayerChar`)))
      (set `self.SkillTime` 0.0)
      (`self.PlayAnimMontage` "/Game/HellDemonBoss/Montage/Boss_HellDemon_Sweeping_Montage.Boss_HellDemon_Sweeping_Montage" 1.0 "Start")
      (else
        (set `self.isSkill` false)
        (set `self.isNormal` true)
        (set `self.CurState` "NewEnumerator2")
        (`self.K2_SetActorRotation` (`KismetMathLibrary.Conv_VectorToRotator` (`self.DirToPlayerChar`)))
        (`self.PlayAnimMontage` "/Game/HellDemonBoss/Montage/Boss_HellDemon_NormalAttack_Montage.Boss_HellDemon_NormalAttack_Montage")))))

(event `charReTarget`
  (bind _returnvalue (`GameplayStatics.GetPlayerCharacter` 0))
  (bind _returnvalue_2 (`KismetMathLibrary.MakeVector` (.x (- (`self.K2_GetActorLocation` _returnvalue) (`self.K2_GetActorLocation`))) (.y (- (`self.K2_GetActorLocation` _returnvalue) (`self.K2_GetActorLocation`))) (.z (- (`self.K2_GetActorLocation` _returnvalue) (`self.K2_GetActorLocation`)))))
  (set `self.aiAttack` false)
  (if (`self.isMove`)
    (bind _asblade_bp (cast `/Game/BLADE/BladeBP` _returnvalue))
    (set `self.IsDeathPlayerChar` (`/Game/BLADE/BladeBP.IsDeath` _asblade_bp))
    (set `self.DistancePlayerChar` (`KismetMathLibrary.VSize` _returnvalue_2))
    (set `self.DirToPlayerChar` (`KismetMathLibrary.Normal` _returnvalue_2))))

(event `SaveDisAndDir`
  (bind _returnvalue (`GameplayStatics.GetPlayerCharacter` 0))
  (bind _returnvalue_2 (`KismetMathLibrary.MakeVector` (.x (- (`self.K2_GetActorLocation` _returnvalue) (`self.K2_GetActorLocation`))) (.y (- (`self.K2_GetActorLocation` _returnvalue) (`self.K2_GetActorLocation`))) (.z (- (`self.K2_GetActorLocation` _returnvalue) (`self.K2_GetActorLocation`)))))
  (set `self.aiAttack` false)
  (if (`self.isMove`)
    (bind _asblade_bp (cast `/Game/BLADE/BladeBP` _returnvalue))
    (set `self.IsDeathPlayerChar` (`/Game/BLADE/BladeBP.IsDeath` _asblade_bp))
    (set `self.DistancePlayerChar` (`KismetMathLibrary.VSize` _returnvalue_2))
    (set `self.DirToPlayerChar` (`KismetMathLibrary.Normal` _returnvalue_2))))

(event `Aitarget`
  (set `self.aiAttack` true)
  (if (`self.isMove`)
    (bind _returnvalue (`GameplayStatics.GetActorOfClass` "/Game/AI/Aiblade.Aiblade_C"))
    (if (`/Game/AI/Aiblade.isdeathai` _returnvalue)
      (`/Engine/EditorBlueprintResources/StandardMacros.DoOnce` false
        (:`Completed`
          (`KismetSystemLibrary.PrintString` "ai사망")
          (set `self.ischcool` true)))
      (else
        (bind _returnvalue_2 (`KismetMathLibrary.MakeVector` (.x (- (`self.K2_GetActorLocation` _returnvalue) (`self.K2_GetActorLocation`))) (.y (- (`self.K2_GetActorLocation` _returnvalue) (`self.K2_GetActorLocation`))) (.z (- (`self.K2_GetActorLocation` _returnvalue) (`self.K2_GetActorLocation`)))))
        (set `self.DistancePlayerChar` (`KismetMathLibrary.VSize` _returnvalue_2))
        (set `self.DirToPlayerChar` (`KismetMathLibrary.Normal` _returnvalue_2))))))

(event `self.ReceiveAnyDamage`
  (params (Damage :type "Float (single-precision)") (DamageType :type "DamageType Object Reference") (InstigatedBy :type "Controller Object Reference") (DamageCauser :type "Actor Object Reference"))
  (if (not (`self.isNoDamage`))
    (bind _output_get (set `self.Hp` (- (`self.Hp`) Damage)))
    (`/Game/Blueprints/Widgets/GamePlayMainWidget.Update_BossHPBar` (`/Game/Blueprints/SideScrollGameInstance.gwmg` (`self.SideScrollGameRef`)) (`self.Hp`) (`self.MaxHp`))
    (`self.ChangeDamageColor`)
    (if (<= _output_get 0.0)
      (`self.PlayAnimMontage` "/Game/HellDemonBoss/Montage/Boss_HellDemon_Death_Montage.Boss_HellDemon_Death_Montage")
      (`KismetSystemLibrary.PrintString` "사망")
      (set `self.isDeathBoss` true)
      (set `self.CurState` "NewEnumerator4")
      (`PrimitiveComponent.SetCollisionEnabled` (`self.CapsuleComponent`) "NoCollision")
      (`PrimitiveComponent.SetCollisionEnabled` (`self.Capsule`) "NoCollision")
      (`PrimitiveComponent.SetCollisionEnabled` (`self.CapsuleR`) "NoCollision")
      (`KismetSystemLibrary.Delay` 2.0)
      (`GameplayStatics.PlaySound2D` "/Game/Assets/Sound/Others/_Track_03__Boom_Sound_Effect._Track_03__Boom_Sound_Effect" 1.0 1.0 0.0 null null)
      (`NiagaraFunctionLibrary.SpawnSystemAtLocation` "/Game/Assets/VFX/Niagara/New_Effects/VFX_HellDemon_Kill.VFX_HellDemon_Kill" (`SceneComponent.K2_GetComponentLocation` (`self.Mesh`)))
      (`self.K2_DestroyActor`))))

(event `ChangeDamageColor`
  (`GameplayStatics.SpawnEmitterAttached` null (`self.CapsuleComponent`))
  (`PrimitiveComponent.SetMaterial` (`self.Mesh`) 0 null)
  (`KismetSystemLibrary.Delay` 0.2)
  (`PrimitiveComponent.SetMaterial` (`self.Mesh`) 0 "/Game/Assets/Material/MM_Asphalt2.MM_Asphalt2")
  (`PrimitiveComponent.SetMaterial` (`self.Mesh`) 1 "/Game/Assets/Material/MM_Lava2_2.MM_Lava2_2"))

(event `self.CapsuleR.OnComponentBeginOverlap`
  (params (OverlappedComponent :type "PrimitiveComponent Object Reference") (OtherActor :type "Actor Object Reference") (OtherComp :type "PrimitiveComponent Object Reference") (OtherBodyIndex :type Integer) (bFromSweep :type Boolean) (SweepResult :type "HitResult Structure (by ref)"))
  (if (!= OtherActor self)
    (if (!= (`|GetArrayItem` (`self.Tags`)) (`|GetArrayItem` (`Actor.Tags` OtherActor)))
      (if (== (`|GetArrayItem` (`ActorComponent.ComponentTags` OtherComp) 2) "mainChar")
        (if (`self.isNormal`)
          (if (not (`self.isSkill`))
            (`GameplayStatics.ApplyDamage` OtherActor (`self.Atk`) null self)
            (bind _output_get (set `self.AttackDamage` (+ (`self.AttackDamage`) 10.0)))))))))

(event `self.Capsule.OnComponentBeginOverlap`
  (params (OverlappedComponent :type "PrimitiveComponent Object Reference") (OtherActor :type "Actor Object Reference") (OtherComp :type "PrimitiveComponent Object Reference") (OtherBodyIndex :type Integer) (bFromSweep :type Boolean) (SweepResult :type "HitResult Structure (by ref)"))
  (if (!= OtherActor self)
    (if (!= (`|GetArrayItem` (`self.Tags`)) (`|GetArrayItem` (`Actor.Tags` OtherActor)))
      (if (== (`|GetArrayItem` (`ActorComponent.ComponentTags` OtherComp) 2) "mainChar")
        (if (`self.isNormal`)
          _
          (elif (`self.isSkill`)
            (`GameplayStatics.ApplyDamage` OtherActor (`self.Skill1Atk`) null self)
            (bind _output_get (set `self.skillDamage` (+ (`self.skillDamage`) 30.0)))))))))

(event `OnColStart_Attack`
  (`PrimitiveComponent.SetCollisionEnabled` (`self.CapsuleR`) "QueryAndPhysics"))

(event `OnColEnd_Attack`
  (`PrimitiveComponent.SetCollisionEnabled` (`self.CapsuleR`) "NoCollision"))

(event `OnColStart_Skill1Attack`
  (`PrimitiveComponent.SetCollisionEnabled` (`self.Capsule`) "QueryAndPhysics"))

(event `OnColEnd_Skill1Attack`
  (`PrimitiveComponent.SetCollisionEnabled` (`self.Capsule`) "NoCollision"))

(fn `UserConstructionScript`)