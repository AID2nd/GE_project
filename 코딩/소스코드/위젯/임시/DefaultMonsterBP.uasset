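; Default goblin monster character that chases and slashes the player along the world Y axis, idling when the player dies or the stage clears.
; Tick caches player distance and direction, then drives an enum state machine from idle through follow to attack, repeating slashes on animation end.
; Attack events toggle a hit capsule that damages character components with differing actor tags.
; Damage updates a spawned HP bar actor, flashes the material, and handles death with delayed destruction.
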(event `self.ReceiveBeginPlay`
  (bind _returnvalue (`|SpawnActorFromClass` "/Game/Blueprints/HpBarBP.HpBarBP_C" (`KismetMathLibrary.MakeTransform` (`SceneComponent.K2_GetComponentLocation` (`self.CubeLocation`))) "Undefined" "OverrideRootScale" null null))
  (set `self.HpBarActor` _returnvalue))

(event `self.ReceiveTick`
  (params (DeltaSeconds :type "Float (single-precision)"))
  (bind _hpbaractor (`self.HpBarActor`))
  (`self.SaveDisAndDir`)
  (`/Engine/EditorBlueprintResources/StandardMacros.IsValid` _hpbaractor
    (:`Is Valid`
      (`/Game/Blueprints/HpBarBP.UpdateLocation` _hpbaractor (`SceneComponent.K2_GetComponentLocation` (`self.CubeLocation`))))
    (:`Is Not Valid`
      _))
  (if (or (`self.IsDeathPlayerChar`) (`self.IsStageClear`))
    (set `self.CurState` "NewEnumerator3"))
  (switch `/Game/Enums/MonsterState` (`self.CurState`)
    (:`NewEnumerator0`
      (if (<= (`self.DistancePlayerChar`) 500.0)
        (set `self.CurState` "NewEnumerator1")))
    (:`NewEnumerator1`
      (if (<= (`self.DistancePlayerChar`) 160.0)
        (set `self.CurState` "NewEnumerator2")
        (`self.PlayAnimMontage` "/Game/Mesh/Monster/Animations/golblin_slash_Montage.golblin_slash_Montage")
        (set `self.IsAttacking` true)
        (else
          (`self.AddMovementInput` (`self.DirToPlayerChar`)))))
    (:`NewEnumerator2`
      (if (`self.IsAttacking`)
        _
        (elif (> (`self.DistancePlayerChar`) 180.0)
          (set `self.CurState` "NewEnumerator1"))))))

(event `OnAnimEnd_Attack`
  (set `self.IsAttacking` false)
  (if (or (`self.IsDeathPlayerChar`) (`self.IsStageClear`))
    (set `self.CurState` "NewEnumerator3")
    (elif (> (`self.DistancePlayerChar`) 180.0)
      (set `self.CurState` "NewEnumerator1")
      (else
        (`self.K2_SetActorRotation` (`KismetMathLibrary.Conv_VectorToRotator` (`self.DirToPlayerChar`)))
        (`self.PlayAnimMontage` "/Game/Mesh/Monster/Animations/golblin_slash_Montage.golblin_slash_Montage")
        (set `self.IsAttacking` true)))))

(event `SaveDisAndDir`
  (bind _returnvalue (`GameplayStatics.GetPlayerCharacter` 0))
  (bind _returnvalue_2 (`KismetMathLibrary.MakeVector` 0.0 (.y (- (`self.K2_GetActorLocation` _returnvalue) (`self.K2_GetActorLocation`)))))
  (bind _asdefault_play_game_mode (cast `/Game/Blueprints/DefaultPlayGameMode` (`GameplayStatics.GetGameMode`)))
  (set `self.IsStageClear` (`|EnumEquality` (`/Game/Blueprints/DefaultPlayGameMode.CurGamePlayState` _asdefault_play_game_mode) "NewEnumerator0"))
  (bind _aspaladin_hero_bp (cast `/Game/Blueprints/Widgets/임시/PaladinHeroBP` _returnvalue))
  (set `self.IsDeathPlayerChar` (`/Game/Blueprints/Widgets/임시/PaladinHeroBP.IsDeath` _aspaladin_hero_bp))
  (set `self.DistancePlayerChar` (`KismetMathLibrary.VSize` _returnvalue_2))
  (set `self.DirToPlayerChar` (`KismetMathLibrary.Normal` _returnvalue_2)))

(event `self.ReceiveAnyDamage`
  (params (Damage :type "Float (single-precision)") (DamageType :type "DamageType Object Reference") (InstigatedBy :type "Controller Object Reference") (DamageCauser :type "Actor Object Reference"))
  (bind _output_get (set `self.Hp` (- (`self.Hp`) Damage)))
  (`/Game/Blueprints/HpBarBP.UpdateMaxHpBar` (`self.HpBarActor`) (`self.Hp`) (`self.MaxHp`))
  (`self.ChangeDamageColor`)
  (if (<= _output_get 0.0)
    (`self.PlayAnimMontage` "/Game/Mesh/Monster/AnimMontage/goblin_death_Montage.goblin_death_Montage")
    (set `self.CurState` "NewEnumerator4")
    (`self.K2_DestroyActor` (`self.HpBarActor`))
    (`KismetSystemLibrary.Delay` 5.0)
    (`self.K2_DestroyActor`)))

(event `ChangeDamageColor`
  (`GameplayStatics.SpawnEmitterAttached` "/Game/InfinityBladeEffects/Effects/FX_Mobile/Fire/combat/P_FireBall_Powerup.P_FireBall_Powerup" (`self.CapsuleComponent`))
  (`PrimitiveComponent.SetMaterial` (`self.Mesh`) 0 "/Game/Mesh/Monster/phong1_Inst.phong1_Inst")
  (`KismetSystemLibrary.Delay` 0.2)
  (`PrimitiveComponent.SetMaterial` (`self.Mesh`) 0 "/Game/Mesh/Monster/phong1.phong1"))

(event `self.Capsule.OnComponentBeginOverlap`
  (params (OverlappedComponent :type "PrimitiveComponent Object Reference") (OtherActor :type "Actor Object Reference") (OtherComp :type "PrimitiveComponent Object Reference") (OtherBodyIndex :type Integer) (bFromSweep :type Boolean) (SweepResult :type "HitResult Structure (by ref)"))
  (if (!= OtherActor self)
    (if (!= (`|GetArrayItem` (`self.Tags`)) (`|GetArrayItem` (`Actor.Tags` OtherActor)))
      (if (== (`|GetArrayItem` (`ActorComponent.ComponentTags` OtherComp)) "Character")
        (`GameplayStatics.ApplyDamage` OtherActor (`self.Atk`) null self)))))

(event `OnColStart_Attack`
  (`PrimitiveComponent.SetCollisionEnabled` (`self.Capsule`) "QueryAndPhysics"))

(event `OnColEnd_Attack`
  (`PrimitiveComponent.SetCollisionEnabled` (`self.Capsule`) "NoCollision"))

(fn `UserConstructionScript`)