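; BP_ExtraFloor is an obstacle floor that slides along the world Y axis according to a PlayerOnButton flag.
; BeginPlay stores the starting Y, and Tick steps the actor toward negative Y while the flag is set and its offset check exceeds FloorDestination.
; With the flag clear, it steps toward positive Y unconditionally, only updating that check against zero.
; Movement is a fixed per-frame teleport-free offset without sweep or delta-time scaling.
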(event `self.ReceiveBeginPlay`
  (bind (_returnvalue_x _returnvalue_y) (`KismetMathLibrary.BreakVector` (`self.K2_GetActorLocation`)))
  (set `self.Floor Location` _returnvalue_y))

(event `self.ReceiveTick`
  (params (DeltaSeconds :type "Float (single-precision)"))
  (bind (_returnvalue_x _returnvalue_y) (`KismetMathLibrary.BreakVector` (`self.K2_GetActorLocation`)))
  (bind (_returnvalue_x_2 _returnvalue_y_2) (`KismetMathLibrary.BreakVector` (`self.K2_GetActorLocation`)))
  (if (`self.Player On Button`)
    (if (`self.Floor Location Check`)
      (`self.K2_SetActorLocation` (+ (`self.K2_GetActorLocation`) (0.0 -10.0 0.0)))
      (set `self.Floor Location Check` (> (- _returnvalue_y (`self.Floor Location`)) (`self.Floor Destination`))))
    (else
      (`self.K2_SetActorLocation` (+ (`self.K2_GetActorLocation`) (0.0 10.0 0.0)))
      (set `self.Floor Location Check` (> (- _returnvalue_y_2 (`self.Floor Location`)) 0.0)))))

(fn `UserConstructionScript`)