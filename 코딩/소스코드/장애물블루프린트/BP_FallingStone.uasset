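; Falling-rock obstacle that quits the game when its mesh hits BladeBP.
; While CheckPlayer is true, Tick drops it with randomly growing downward speed and destroys it below a height limit.
; A hidden red warning light moves down until overlapping BladeBP, while collision volumes toggle a flag and play a sound.
; The chain that flashes the warning and sets CheckPlayer is disconnected, so nothing here starts the fall.
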(event `self.ReceiveBeginPlay`
  (set `self.Gravity` -1.0)
  (set `self.Red Light Speed` -30.0)
  (`SceneComponent.SetHiddenInGame` (`self.Red Light Warning`) true false))

(event `self.ReceiveTick`
  (params (DeltaSeconds :type "Float (single-precision)"))
  (bind (_returnvalue_x _returnvalue_y _returnvalue_z) (`KismetMathLibrary.BreakVector` (`self.K2_GetActorLocation`)))
  (bind _returnvalue (+ (`self.Gravity`) (`KismetMathLibrary.RandomFloatInRange` -0.8 -0.3)))
  (`SceneComponent.K2_AddLocalOffset` (`self.Red Light Warning`) (`KismetMathLibrary.MakeVector` 0.0 0.0 (`self.Red Light Speed`)) false false)
  (if (`self.Check Player`)
    (`self.K2_SetActorLocation` (+ (`self.K2_GetActorLocation`) (`KismetMathLibrary.MakeVector` 0.0 0.0 _returnvalue)))
    (set `self.Gravity` _returnvalue)
    (if (< _returnvalue_z -2000.0)
      (`self.K2_DestroyActor`))))

(event `self.RockCollision.OnComponentBeginOverlap`
  (params (OverlappedComponent :type "PrimitiveComponent Object Reference") (OtherActor :type "Actor Object Reference") (OtherComp :type "PrimitiveComponent Object Reference") (OtherBodyIndex :type Integer) (bFromSweep :type Boolean) (SweepResult :type "HitResult Structure (by ref)"))
  (cast `/Game/blade/BladeBP` OtherActor)
  (set `self.Component Collision` true)
  (`GameplayStatics.PlaySoundAtLocation` null (`self.K2_GetActorLocation`) (struct) 1.0 1.0 0.0 null null null null))

(event `self.CheckPlayerCollision.OnComponentBeginOverlap`
  (params (OverlappedComponent :type "PrimitiveComponent Object Reference") (OtherActor :type "Actor Object Reference") (OtherComp :type "PrimitiveComponent Object Reference") (OtherBodyIndex :type Integer) (bFromSweep :type Boolean) (SweepResult :type "HitResult Structure (by ref)"))
  (cast `/Game/blade/BladeBP` OtherActor
    (:`then`
      (set `self.Component Collision` false))
    (:`CastFailed`
      _))
  (cast `/Game/blade/BladeBP` OtherActor))

(event `self.StaticMeshComponent.OnComponentHit`
  (params (HitComponent :type "PrimitiveComponent Object Reference") (OtherActor :type "Actor Object Reference") (OtherComp :type "PrimitiveComponent Object Reference") (NormalImpulse :type "Vector Structure") (Hit :type "HitResult Structure (by ref)"))
  (cast `/Game/blade/BladeBP` OtherActor)
  (`KismetSystemLibrary.QuitGame` null "Quit"))

(event `self.Red Light Warning.OnComponentBeginOverlap`
  (params (OverlappedComponent :type "PrimitiveComponent Object Reference") (OtherActor :type "Actor Object Reference") (OtherComp :type "PrimitiveComponent Object Reference") (OtherBodyIndex :type Integer) (bFromSweep :type Boolean) (SweepResult :type "HitResult Structure (by ref)"))
  (bind _red_light_warning (`self.Red Light Warning`))
  (cast `/Game/blade/BladeBP` OtherActor)
  (set `self.Red Light Speed` 0.0)
  (`SceneComponent.K2_SetWorldLocation` _red_light_warning (`SceneComponent.K2_GetComponentLocation` _red_light_warning) false false))

(fn `UserConstructionScript`)