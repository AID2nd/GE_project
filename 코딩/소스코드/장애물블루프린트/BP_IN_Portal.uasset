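; BP_IN_Portal is a single-use entrance portal that teleports the BladeBP actor to a paired exit portal.
; On Box overlap, it casts to BladeBP, moves it to the PortalOut Box's world location without sweeping, plays a teleport sound and destroys itself.
; A PlayerInPortal flag follows overlap begin and end for any actor, as it is set before the cast.
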(event `self.Box.OnComponentBeginOverlap`
  (params (OverlappedComponent :type "PrimitiveComponent Object Reference") (OtherActor :type "Actor Object Reference") (OtherComp :type "PrimitiveComponent Object Reference") (OtherBodyIndex :type Integer) (bFromSweep :type Boolean) (SweepResult :type "HitResult Structure (by ref)"))
  (set `self.Player In Portal?` true)
  (bind _asblade_bp (cast `/Game/BLADE/BladeBP` OtherActor))
  (`self.K2_SetActorLocation` _asblade_bp (`SceneComponent.K2_GetComponentLocation` (`/Game/BLUEPRINT/BP_Out_Portalmiddle.Box` (`self.PortalOut`))) false false)
  (`GameplayStatics.PlaySoundAtLocation` "/Game/Assets/Sound/Others/teleport.teleport" (`self.K2_GetActorLocation`) (struct) 1.0 1.0 0.0 null null null null)
  (`self.K2_DestroyActor`))

(event `self.Box.OnComponentEndOverlap`
  (params (OverlappedComponent :type "PrimitiveComponent Object Reference") (OtherActor :type "Actor Object Reference") (OtherComp :type "PrimitiveComponent Object Reference") (OtherBodyIndex :type Integer))
  (set `self.Player In Portal?` false))

(fn `UserConstructionScript`)