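; BP_Moving_FlatBox_AxisX is a moving box actor that shuttles back and forth along the world X axis.
; BeginPlay stores its starting X, and each Tick offsets it by a random step, so speed varies and depends on frame rate.
; BoxLocationCheck flips the direction, sending it back once it passes BoxDestination beyond the start and forward again once it returns.
; Movement uses SetActorLocation without sweep.
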(event `self.ReceiveBeginPlay`
  (bind _returnvalue_x (`KismetMathLibrary.BreakVector` (`self.K2_GetActorLocation`)))
  (set `self.Box Location` _returnvalue_x))

(event `self.ReceiveTick`
  (params (DeltaSeconds :type "Float (single-precision)"))
  (bind _returnvalue_x (`KismetMathLibrary.BreakVector` (`self.K2_GetActorLocation`)))
  (bind _returnvalue_x_2 (`KismetMathLibrary.BreakVector` (`self.K2_GetActorLocation`)))
  (if (`self.Box Location Check`)
    (`self.K2_SetActorLocation` (+ (`self.K2_GetActorLocation`) (`KismetMathLibrary.MakeVector` (`KismetMathLibrary.RandomFloatInRange` -7.0 -5.0))))
    (set `self.Box Location Check` (> (- _returnvalue_x (`self.Box Location`)) 0.0))
    (else
      (`self.K2_SetActorLocation` (+ (`self.K2_GetActorLocation`) (`KismetMathLibrary.MakeVector` (`KismetMathLibrary.RandomFloatInRange` 5.0 7.0))))
      (set `self.Box Location Check` (> (- _returnvalue_x_2 (`self.Box Location`)) (`self.Box Destination`))))))

(fn `UserConstructionScript`)