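; BP_Moving_FlatBox_AxisY is an obstacle box that shuttles back and forth along the world Y axis.
; BeginPlay records the starting Y, and Tick uses the BoxLocationCheck flag to pick the direction.
; The flag flips at a fixed negative offset from the start and at the BoxDestination offset on the return.
; Each frame moves a random step without sweep or delta-time scaling, so speed is jittery and frame-rate dependent.
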(event `self.ReceiveBeginPlay`
  (bind (_returnvalue_x _returnvalue_y) (`KismetMathLibrary.BreakVector` (`self.K2_GetActorLocation`)))
  (set `self.Box Location` _returnvalue_y))

(event `self.ReceiveTick`
  (params (DeltaSeconds :type "Float (single-precision)"))
  (bind (_returnvalue_x _returnvalue_y) (`KismetMathLibrary.BreakVector` (`self.K2_GetActorLocation`)))
  (bind (_returnvalue_x_2 _returnvalue_y_2) (`KismetMathLibrary.BreakVector` (`self.K2_GetActorLocation`)))
  (if (`self.Box Location Check`)
    (`self.K2_SetActorLocation` (+ (`self.K2_GetActorLocation`) (`KismetMathLibrary.MakeVector` 0.0 (`KismetMathLibrary.RandomFloatInRange` -5.0 -15.0))))
    (set `self.Box Location Check` (> (- _returnvalue_y_2 (`self.Box Location`)) -800.0))
    (else
      (`self.K2_SetActorLocation` (+ (`self.K2_GetActorLocation`) (`KismetMathLibrary.MakeVector` 0.0 (`KismetMathLibrary.RandomFloatInRange` 5.0 15.0))))
      (set `self.Box Location Check` (> (- _returnvalue_y (`self.Box Location`)) (`self.Box Destination`))))))

(fn `UserConstructionScript`)