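; Moving thorn wall obstacle that cycles along world X and sets IsDeath on a BladeBP that overlaps its Box.
; Tick runs a ModeSwitch state machine: pause, creep back behind the start, lunge forward past WallDestination, pause, then retreat more slowly.
; Movement is a fixed or random per-frame offset without sweep or delta time, with Delay nodes inside Tick providing the randomized pauses and stuttered wind-up.
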(event `self.ReceiveBeginPlay`
  (bind _returnvalue_x (`KismetMathLibrary.BreakVector` (`self.K2_GetActorLocation`)))
  (set `self.Wall Location` _returnvalue_x))

(event `self.ReceiveTick`
  (params (DeltaSeconds :type "Float (single-precision)"))
  (bind _returnvalue_x (`KismetMathLibrary.BreakVector` (`self.K2_GetActorLocation`)))
  (bind _returnvalue_x_2 (`KismetMathLibrary.BreakVector` (`self.K2_GetActorLocation`)))
  (bind _returnvalue_x_3 (`KismetMathLibrary.BreakVector` (`self.K2_GetActorLocation`)))
  (bind _returnvalue_x_4 (`KismetMathLibrary.BreakVector` (`self.K2_GetActorLocation`)))
  (switch `int` (`self.Mode Switch`)
    (:`0`
      (if (> _returnvalue_x_3 (`self.Wall Location`))
        (`KismetSystemLibrary.Delay` (`KismetMathLibrary.RandomFloatInRange` 1.0 2.0))
        (set `self.Mode Switch` 2)
        (else
          (`KismetSystemLibrary.Delay` (`KismetMathLibrary.RandomFloatInRange` 1.0 2.0))
          (set `self.Mode Switch` 3))))
    (:`1`
      (`self.K2_SetActorLocation` (+ (`self.K2_GetActorLocation`) (40.0 0.0 0.0)))
      (if (> (- _returnvalue_x_2 (`self.Wall Location`)) (`self.Wall Destination`))
        (set `self.Mode Switch` 0)))
    (:`2`
      (`self.K2_SetActorLocation` (+ (`self.K2_GetActorLocation`) (-20.0 0.0 0.0)))
      (if (> (`self.Wall Location`) _returnvalue_x)
        (set `self.Mode Switch` 0)))
    (:`3`
      (`KismetSystemLibrary.Delay` 0.1)
      (`self.K2_SetActorLocation` (+ (`self.K2_GetActorLocation`) (`KismetMathLibrary.MakeVector` (`KismetMathLibrary.RandomFloatInRange` -10.0 -5.0))))
      (if (> (- (`self.Wall Location`) _returnvalue_x_4) 70.0)
        (set `self.Mode Switch` 1)))))

(event `self.Box.OnComponentBeginOverlap`
  (params (OverlappedComponent :type "PrimitiveComponent Object Reference") (OtherActor :type "Actor Object Reference") (OtherComp :type "PrimitiveComponent Object Reference") (OtherBodyIndex :type Integer) (bFromSweep :type Boolean) (SweepResult :type "HitResult Structure (by ref)"))
  (bind _asblade_bp (cast `/Game/BLADE/BladeBP` OtherActor))
  (set `/Game/BLADE/BladeBP.IsDeath` true _asblade_bp))

(fn `UserConstructionScript`)