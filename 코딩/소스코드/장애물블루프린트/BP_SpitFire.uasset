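; Spitting fire obstacle that repeatedly travels along world +Y and quits the game when its capsule overlaps the BladeBP actor.
; Tick moves it a fixed step per frame, so speed depends on frame rate, until its offset from the BeginPlay Y position exceeds FireDestination.
; FireLocationCheck then switches Tick to a Delay that holds it briefly before snapping Y back to the start and restarting the run.
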(event `self.ReceiveBeginPlay`
  (bind (_returnvalue_x _returnvalue_y) (`KismetMathLibrary.BreakVector` (`self.K2_GetActorLocation`)))
  (set `self.Start Location` _returnvalue_y))

(event `self.ReceiveTick`
  (params (DeltaSeconds :type "Float (single-precision)"))
  (bind (_returnvalue_x _returnvalue_y) (`KismetMathLibrary.BreakVector` (`self.K2_GetActorLocation`)))
  (bind (_returnvalue_x_2 _returnvalue_y_2 _returnvalue_z) (`KismetMathLibrary.BreakVector` (`self.K2_GetActorLocation`)))
  (if (`self.Fire Location Check`)
    (`KismetSystemLibrary.Delay` 5.0)
    (`self.K2_SetActorLocation` (`KismetMathLibrary.MakeVector` _returnvalue_x_2 (`self.Start Location`) _returnvalue_z))
    (set `self.Fire Location Check` false)
    (else
      (`self.K2_SetActorLocation` (+ (`self.K2_GetActorLocation`) (0.0 5.0 0.0)))
      (set `self.Fire Location Check` (> (- _returnvalue_y (`self.Start Location`)) (`self.Fire Destination`))))))

(event `self.Capsule.OnComponentBeginOverlap`
  (params (OverlappedComponent :type "PrimitiveComponent Object Reference") (OtherActor :type "Actor Object Reference") (OtherComp :type "PrimitiveComponent Object Reference") (OtherBodyIndex :type Integer) (bFromSweep :type Boolean) (SweepResult :type "HitResult Structure (by ref)"))
  (cast `/Game/blade/BladeBP` OtherActor)
  (`KismetSystemLibrary.QuitGame` null "Quit"))

(fn `UserConstructionScript`)