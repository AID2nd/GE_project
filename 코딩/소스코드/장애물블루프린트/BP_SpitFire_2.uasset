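; BP_SpitFire_2 is an obstacle that fails the stage when the BladeBP actor touches it.
; Its Capsule overlap casts to BladeBP, then adds a StageFail widget to the viewport, shows the mouse cursor and disables player character input.
; BeginPlay saves the actor's Y position in StartLocation, which nothing here reads, and Tick is empty, so this graph drives no movement.
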(event `self.ReceiveBeginPlay`
  (bind (_returnvalue_x _returnvalue_y) (`KismetMathLibrary.BreakVector` (`self.K2_GetActorLocation`)))
  (set `self.Start Location` _returnvalue_y))

(event `self.ReceiveTick`
  (params (DeltaSeconds :type "Float (single-precision)")))

(event `self.Capsule.OnComponentBeginOverlap`
  (params (OverlappedComponent :type "PrimitiveComponent Object Reference") (OtherActor :type "Actor Object Reference") (OtherComp :type "PrimitiveComponent Object Reference") (OtherBodyIndex :type Integer) (bFromSweep :type Boolean) (SweepResult :type "HitResult Structure (by ref)"))
  (bind _returnvalue (`GameplayStatics.GetPlayerController` 0))
  (cast `/Game/BLADE/BladeBP` OtherActor)
  (bind _returnvalue_2 (`|CreateWidget` "/Game/Blueprints/Widgets/StageFail.StageFail_C" _returnvalue))
  (`UserWidget.AddToViewport` _returnvalue_2 0)
  (set `PlayerController.bShowMouseCursor` true _returnvalue)
  (`self.DisableInput` (`GameplayStatics.GetPlayerCharacter` 0) (`GameplayStatics.GetPlayerController` 0)))

(fn `UserConstructionScript`)