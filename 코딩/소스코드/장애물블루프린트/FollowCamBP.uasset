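; FollowCamBP is a follow-camera actor that trails player character 0 at the offset captured on BeginPlay.
; Each Tick it lerps its location toward the player's position plus that offset, using DeltaSeconds times Smooth as alpha.
; A BladeBP death check runs afterward but has no effect, and the spawn, view-target and game-instance nodes are unconnected leftovers that never run.
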(event `self.ReceiveBeginPlay`
  (set `self.Offset` (- (`self.K2_GetActorLocation`) (`self.K2_GetActorLocation` (`GameplayStatics.GetPlayerCharacter` 0)))))

(event `self.ReceiveTick`
  (params (DeltaSeconds :type "Float (single-precision)"))
  (`self.K2_SetActorLocation` (`KismetMathLibrary.VLerp` (`self.K2_GetActorLocation`) (+ (`self.K2_GetActorLocation` (`GameplayStatics.GetPlayerCharacter` 0)) (`self.Offset`)) (* DeltaSeconds (`self.Smooth`))))
  (bind _asblade_bp (cast `/Game/blade/BladeBP` (`GameplayStatics.GetPlayerCharacter` 0)))
  (if (`/Game/blade/BladeBP.IsDeath` _asblade_bp)
    _))

(fn `UserConstructionScript`)