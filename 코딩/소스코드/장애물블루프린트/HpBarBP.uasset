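; HpBarBP is an actor that displays a health bar through a widget component.
; On BeginPlay it casts the component's widget to CharHpBar and caches its progress bar.
; UpdateLocation moves the actor to a given position, and UpdateMaxHpBar sets the bar's fill to Hp divided by MaxHp.
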(event `self.ReceiveBeginPlay`
  (bind _aschar_hp_bar (cast `/Game/Blueprints/Widgets/charHpBar` (`WidgetComponent.GetUserWidgetObject` (`self.HpBarWidget`))))
  (set `self.BP_HpBar` (`/Game/Blueprints/Widgets/charHpBar.ProgressBar_41` _aschar_hp_bar)))

(fn `UpdateLocation`
  (params (Location :type "Vector Structure"))
  (`self.K2_SetActorLocation` Location))

(fn `UpdateMaxHpBar`
  (params (Hp :type "Float (double-precision)") (MaxHp :type "Float (double-precision)"))
  (`ProgressBar.SetPercent` (`self.BP_HpBar`) (/ Hp MaxHp)))

(fn `UserConstructionScript`)