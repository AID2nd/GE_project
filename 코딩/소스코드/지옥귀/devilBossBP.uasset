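; Golem boss character for a side-scrolling game that chases and attacks the player, updates the boss HP bar and shows stage clear on death.
; Tick caches player distance and direction to drive an idle, follow, attack and death state machine.
; A self-calling Delay timer selects skill over normal attacks, each with random avoid flags.
; Event-toggled capsules apply attack damage; taking damage flashes materials and eventually triggers death.
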(event `self.ReceiveBeginPlay`
  (bind _asside_scroll_game_instance (cast `/Game/Blueprints/SideScrollGameInstance` (`GameplayStatics.GetGameInstance`)))
  (set `self.SideScrollGameRef` _asside_scroll_game_instance)
  (set `self.Hp` 100.0)
  (`/Game/Blueprints/Widgets/GamePlayMainWidget.Update_BossHPBar` (`/Game/Blueprints/SideScrollGameInstance.gwmg` (`self.SideScrollGameRef`)) (`self.Hp`) (`self.MaxHp`)))

(event `SkillTimeLoop`
  (`KismetSystemLibrary.Delay` 1.0)
  (set `self.SkillTime` (+ (`self.SkillTime`) 1.0))
  (`self.SkillTimeLoop`))

(event `self.ReceiveTick`
  (params (DeltaSeconds :type "Float (single-precision)"))
  (bind _returnvalue (`GameplayStatics.GetPlayerController` 0))
  (bind _sidescrollgameref (`self.SideScrollGameRef`))
  (bind _bosstexture (`self.BossTexture`))
  (`self.SaveDisAndDir`)
  (if (`self.IsDeathPlayerChar`)
    (set `self.CurState` "NewEnumerator3"))
  (switch `/Game/Enums/MonsterState` (`self.CurState`)
    (:`NewEnumerator0`
      (if (<= (`self.DistancePlayerChar`) 500.0)
        (`/Game/Blueprints/SideScrollGameInstance.ShowBossUI` _sidescrollgameref true _bosstexture)
        (set `self.CurState` "NewEnumerator1")
        (`self.SkillTimeLoop`)
        (else
          (`/Game/Blueprints/SideScrollGameInstance.ShowBossUI` _sidescrollgameref false _bosstexture))))
    (:`NewEnumerator1`
      (if (<= (`self.DistancePlayerChar`) 130.0)
        (`self.StartAttack`)
        (elif (not (> (`self.DistancePlayerChar`) 1000.0))
          (`self.AddMovementInput` (`self.DirToPlayerChar`)))))
    (:`NewEnumerator2`
      (if (`self.IsAttacking`)
        _
        (elif (> (`self.DistancePlayerChar`) 150.0)
          (set `self.CurState` "NewEnumerator1"))))
    (:`NewEnumerator4`
      (bind _returnvalue_2 (`|CreateWidget` "/Game/Blueprints/Widgets/StageClear.StageClear_C" _returnvalue))
      (`UserWidget.AddToViewport` _returnvalue_2 0)
      (set `PlayerController.bShowMouseCursor` true _returnvalue)
      (`self.DisableInput` (`GameplayStatics.GetPlayerCharacter` 0) (`GameplayStatics.GetPlayerController` 0))
      (`KismetSystemLibrary.Delay` 2.0)
      (`ActorComponent.K2_DestroyComponent` (`self.Mesh`)))))

(event `save`
  (`KismetSystemLibrary.PrintString` "보스제력세이브")
  (set `self.Hp` 100.0)
  (`/Game/Blueprints/Widgets/GamePlayMainWidget.Update_BossHPBar` (`/Game/Blueprints/SideScrollGameInstance.gwmg` (`self.SideScrollGameRef`)) (`self.Hp`) (`self.MaxHp`)))

(event `OnAnimEnd_Attack`
  (set `self.IsAttacking` false)
  (if (`self.IsDeathPlayerChar`)
    (set `self.CurState` "NewEnumerator3")
    (elif (> (`self.DistancePlayerChar`) 180.0)
      (set `self.CurState` "NewEnumerator1")
      (else
        (`self.StartAttack`)))))

(event `StartAttack`
  (set `self.IsAttacking` true)
  (if (>= (`self.SkillTime`) 5.0)
    (set `self.isSkill` true)
    (set `self.isNormal` false)
    (set `self.CurState` "NewEnumerator5")
    (`self.K2_SetActorRotation` (`KismetMathLibrary.Conv_VectorToRotator` (`self.DirToPlayerChar`)))
    (set `self.SkillTime` 0.0)
    (`self.PlayAnimMontage` "/Game/bossMapOb/mainboss/montage/boss_guardian_golem_normalattack_Montage.boss_guardian_golem_normalattack_Montage" 1.0 "Start")
    (if (<= (`KismetMathLibrary.RandomIntegerInRange` 1 100) 25)
      (`KismetSystemLibrary.PrintString` "스킬공격회피")
      (set `self.isAvoidSkill` true))
    (else
      (set `self.isSkill` false)
      (set `self.isNormal` true)
      (set `self.CurState` "NewEnumerator2")
      (`self.K2_SetActorRotation` (`KismetMathLibrary.Conv_VectorToRotator` (`self.DirToPlayerChar`)))
      (`self.PlayAnimMontage` "/Game/bossMapOb/mainboss/montage/boss_guardian_golem_chargeattack_Montage.boss_guardian_golem_chargeattack_Montage")
      (if (<= (`KismetMathLibrary.RandomIntegerInRange` 1 100) 27)
        (`KismetSystemLibrary.PrintString` "일반공격회피")
        (set `self.isAvoidAttack` true)))))

(event `SaveDisAndDir`
  (bind _returnvalue (`GameplayStatics.GetPlayerCharacter` 0))
  (bind _returnvalue_2 (`KismetMathLibrary.MakeVector` (.x (- (`self.K2_GetActorLocation` _returnvalue) (`self.K2_GetActorLocation`))) (.y (- (`self.K2_GetActorLocation` _returnvalue) (`self.K2_GetActorLocation`))) (.z (- (`self.K2_GetActorLocation` _returnvalue) (`self.K2_GetActorLocation`)))))
  (bind _asblade_bp_boss (cast `/Game/bossMapOb/BladeBP_boss` _returnvalue))
  (set `self.IsDeathPlayerChar` (`/Game/bossMapOb/BladeBP_boss.IsDeath` _asblade_bp_boss))
  (set `self.DistancePlayerChar` (`KismetMathLibrary.VSize` _returnvalue_2))
  (set `self.DirToPlayerChar` (`KismetMathLibrary.Normal` _returnvalue_2)))

(event `saveAi`
  (bind _returnvalue (`GameplayStatics.GetPlayerCharacter` 0))
  (bind _returnvalue_2 (`KismetMathLibrary.MakeVector` (.x (- (`self.K2_GetActorLocation` _returnvalue) (`self.K2_GetActorLocation`))) (.y (- (`self.K2_GetActorLocation` _returnvalue) (`self.K2_GetActorLocation`))) (.z (- (`self.K2_GetActorLocation` _returnvalue) (`self.K2_GetActorLocation`)))))
  (cast `/Game/AI/Aiblade` _returnvalue)
  (set `self.DistancePlayerChar` (`KismetMathLibrary.VSize` _returnvalue_2))
  (set `self.DirToPlayerChar` (`KismetMathLibrary.Normal` _returnvalue_2)))

(event `self.ReceiveAnyDamage`
  (params (Damage :type "Float (single-precision)") (DamageType :type "DamageType Object Reference") (InstigatedBy :type "Controller Object Reference") (DamageCauser :type "Actor Object Reference"))
  (bind _output_get (set `self.Hp` (- (`self.Hp`) Damage)))
  (`/Game/Blueprints/Widgets/GamePlayMainWidget.Update_BossHPBar` (`/Game/Blueprints/SideScrollGameInstance.gwmg` (`self.SideScrollGameRef`)) (`self.Hp`) (`self.MaxHp`))
  (`self.ChangeDamageColor`)
  (if (<= _output_get 0.0)
    (`self.PlayAnimMontage` "/Game/bossMapOb/mainboss/montage/boss_guardian_golem_chargelaser_Montage.boss_guardian_golem_chargelaser_Montage")
    (`KismetSystemLibrary.PrintString` "사망")
    (set `self.isDeathBoss` true)
    (set `self.CurState` "NewEnumerator4")
    (`PrimitiveComponent.SetCollisionEnabled` (`self.CapsuleComponent`) "NoCollision")
    (`PrimitiveComponent.SetCollisionEnabled` (`self.Capsule`) "NoCollision")
    (`PrimitiveComponent.SetCollisionEnabled` (`self.CapsuleR`) "NoCollision")
    (`KismetSystemLibrary.Delay` 2.0)
    (`self.K2_DestroyActor`)))

(event `ChangeDamageColor`
  (`GameplayStatics.SpawnEmitterAttached` "/Game/InfinityBladeEffects/Effects/FX_Mobile/Fire/combat/P_FireBall_Powerup.P_FireBall_Powerup" (`self.CapsuleComponent`))
  (`PrimitiveComponent.SetMaterial` (`self.Mesh`) 0 "/Game/InfinityBladeEffects/Effects/FX_Materials/Mobile/Beakable_Master_MeshEmit.Beakable_Master_MeshEmit")
  (`KismetSystemLibrary.Delay` 0.2)
  (`PrimitiveComponent.SetMaterial` (`self.Mesh`) 0 "/Game/Assets/Material/MM_Asphalt2.MM_Asphalt2")
  (`PrimitiveComponent.SetMaterial` (`self.Mesh`) 1 "/Game/Assets/Material/MM_Lava2_2.MM_Lava2_2"))

(event `self.CapsuleR.OnComponentBeginOverlap`
  (params (OverlappedComponent :type "PrimitiveComponent Object Reference") (OtherActor :type "Actor Object Reference") (OtherComp :type "PrimitiveComponent Object Reference") (OtherBodyIndex :type Integer) (bFromSweep :type Boolean) (SweepResult :type "HitResult Structure (by ref)"))
  (if (!= OtherActor self)
    (if (!= (`|GetArrayItem` (`self.Tags`)) (`|GetArrayItem` (`Actor.Tags` OtherActor)))
      (if (== (`|GetArrayItem` (`ActorComponent.ComponentTags` OtherComp) 2) "mainChar")
        (if (`self.isNormal`)
          (if (not (`self.isSkill`))
            (`GameplayStatics.ApplyDamage` OtherActor (`self.Atk`) null self)
            (bind _output_get (set `self.AttackDamage` (+ (`self.AttackDamage`) 10.0)))))))))

(event `self.Capsule.OnComponentBeginOverlap`
  (params (OverlappedComponent :type "PrimitiveComponent Object Reference") (OtherActor :type "Actor Object Reference") (OtherComp :type "PrimitiveComponent Object Reference") (OtherBodyIndex :type Integer) (bFromSweep :type Boolean) (SweepResult :type "HitResult Structure (by ref)"))
  (if (!= OtherActor self)
    (if (!= (`|GetArrayItem` (`self.Tags`)) (`|GetArrayItem` (`Actor.Tags` OtherActor)))
      (if (== (`|GetArrayItem` (`ActorComponent.ComponentTags` OtherComp) 2) "mainChar")
        (if (`self.isNormal`)
          _
          (elif (`self.isSkill`)
            (`GameplayStatics.ApplyDamage` OtherActor (`self.Skill1Atk`) null self)
            (bind _output_get (set `self.skillDamage` (+ (`self.skillDamage`) 30.0)))))))))

(event `OnColStart_Attack`
  (`PrimitiveComponent.SetCollisionEnabled` (`self.CapsuleR`) "QueryAndPhysics"))

(event `OnColEnd_Attack`
  (`PrimitiveComponent.SetCollisionEnabled` (`self.CapsuleR`) "NoCollision"))

(event `OnColStart_Skill1Attack`
  (`PrimitiveComponent.SetCollisionEnabled` (`self.Capsule`) "QueryAndPhysics"))

(event `OnColEnd_Skill1Attack`
  (`PrimitiveComponent.SetCollisionEnabled` (`self.Capsule`) "NoCollision"))

(fn `UserConstructionScript`)