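; Player-controlled cannon shooter character with camera-relative movement, jumping and three ranged attacks.
; Left mouse, T and M each briefly lock movement, play the attack montage and spawn a different projectile from a weapon component.
; Damage updates the game instance's HP bar and flashes the material; death disables input and spawns an Aicannon.
; A separate revive event spawns and possesses an Aiblade, destroying this character's mesh and capsule.
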(event `self.ReceiveBeginPlay`
  (bind _asside_scroll_game_instance (cast `/Game/Blueprints/SideScrollGameInstance` (`GameplayStatics.GetGameInstance`)))
  (set `self.SideScrollGameInsRef` _asside_scroll_game_instance))

(event `self.ReceiveTick`
  (params (DeltaSeconds :type "Float (single-precision)"))
  (`|ExecutionSequence`))

(event `InputAxis|LeftRight`
  (params (AxisValue :type "Float (single-precision)"))
  (if (`self.ismove`)
    (if (not (`self.IsAttacking`))
      (`self.AddMovementInput` (`KismetMathLibrary.GetRightVector` (`KismetMathLibrary.MakeRotator` 0.0 0.0 (.yaw (`self.GetControlRotation`)))) AxisValue))))

(event `Key|LeftMouseButton`
  (params (Key :type "Key Structure"))
  (:`Pressed`
    (set `self.ismove` false)
    (`KismetSystemLibrary.Delay` 0.4)
    (`self.PlayAnimMontage` "/Game/CANNONSHOOTER/montage/cannonshooter_attack_Montage.cannonshooter_attack_Montage")
    (`|SpawnActorFromClass` "/Game/CANNONSHOOTER/cannon_bullet_BP.cannon_bullet_BP_C" (`SceneComponent.K2_GetComponentToWorld` (`self.WeaponSkeletalMesh`)) "Undefined" "OverrideRootScale" null null)
    (`KismetSystemLibrary.Delay` 1.0)
    (set `self.ismove` true)))

(event `InputAxis|ForwardBackward`
  (params (AxisValue :type "Float (single-precision)"))
  (if (`self.ismove`)
    (if (not (`self.IsAttacking`))
      (`self.AddMovementInput` (`KismetMathLibrary.GetForwardVector` (`KismetMathLibrary.MakeRotator` 0.0 0.0 (.yaw (`self.GetControlRotation`)))) AxisValue))))

(event `InputAxis|Turn`
  (params (AxisValue :type "Float (single-precision)"))
  (`self.AddControllerYawInput` AxisValue))

(event `Key|SpaceBar`
  (params (Key :type "Key Structure"))
  (:`Pressed`
    (if (`NavMovementComponent.IsFalling` (`self.CharacterMovement`))
      _
      (elif (not (`self.IsAttacking`))
        (`self.Jump`)
        (`self.PlayAnimMontage` "/Game/CANNONSHOOTER/montage/cannonshooter_jump_Montage.cannonshooter_jump_Montage"))))
  (:`Released`
    (`self.StopJumping`)))

(event `InputAxis|LookUp`
  (params (AxisValue :type "Float (single-precision)"))
  (`self.AddControllerPitchInput` AxisValue))

(event `self.OnLanded`
  (params (Hit :type "HitResult Structure (by ref)"))
  (`self.StopAnimMontage` "/Game/CANNONSHOOTER/montage/cannonshooter_jump_Montage.cannonshooter_jump_Montage"))

(event `Key|T`
  (params (Key :type "Key Structure"))
  (:`Pressed`
    (set `self.ismove` false)
    (`KismetSystemLibrary.Delay` 0.4)
    (`self.PlayAnimMontage` "/Game/CANNONSHOOTER/montage/cannonshooter_attack_Montage.cannonshooter_attack_Montage")
    (`|SpawnActorFromClass` "/Game/CANNONSHOOTER/cannon_bulletSkill1_BP.cannon_bulletSkill1_BP_C" (`SceneComponent.K2_GetComponentToWorld` (`self.WeaponSkeletalMesh`)) "Undefined" "OverrideRootScale" null null)
    (`KismetSystemLibrary.Delay` 1.0)
    (set `self.ismove` true)))

(event `Key|M`
  (params (Key :type "Key Structure"))
  (:`Pressed`
    (set `self.ismove` false)
    (`KismetSystemLibrary.Delay` 0.4)
    (`self.PlayAnimMontage` "/Game/CANNONSHOOTER/montage/cannonshooter_attack_Montage.cannonshooter_attack_Montage")
    (`|SpawnActorFromClass` "/Game/CANNONSHOOTER/cannon_misa_bullet_BP.cannon_misa_bullet_BP_C" (`SceneComponent.K2_GetComponentToWorld` (`self.WeaponSkillMisa`)) "Undefined" "OverrideRootScale" null null)
    (`KismetSystemLibrary.Delay` 1.0)
    (set `self.ismove` true)))

(event `self.ReceiveAnyDamage`
  (params (Damage :type "Float (single-precision)") (DamageType :type "DamageType Object Reference") (InstigatedBy :type "Controller Object Reference") (DamageCauser :type "Actor Object Reference"))
  (bind _output_get (set `self.Hp` (- (`self.Hp`) Damage)))
  (`/Game/Blueprints/Widgets/임시/GamePlayMain.Update_HeroHPBar` (`/Game/Blueprints/SideScrollGameInstance.GamePlayMainWidgetRef` (`self.SideScrollGameInsRef`)) (`self.Hp`) (`self.MaxHp`))
  (`self.ChangeDamageColor`)
  (if (<= _output_get 0.0)
    (`self.PlayAnimMontage` "/Game/CANNONSHOOTER/montage/cannonshooter_death_Montage.cannonshooter_death_Montage")
    (set `self.IsDeath` true)
    (`self.DisableInput` null)
    (`KismetSystemLibrary.Delay` 2.0)
    (`|SpawnActorFromClass` "/Game/CANNONSHOOTER/Aicannon.Aicannon_C" (`self.GetTransform`) "AlwaysSpawn" "OverrideRootScale" null null)
    (bind _asside_scroll_game_instance (cast `/Game/Blueprints/SideScrollGameInstance` (`GameplayStatics.GetGameInstance`)))
    (set `self.SideScrollGameInsRef` _asside_scroll_game_instance)))

(event `ChangeDamageColor`
  (`PrimitiveComponent.SetMaterial` (`self.Mesh`) 0 "/Game/Mesh/Paladin/Paladin_MAT_Inst.Paladin_MAT_Inst")
  (`KismetSystemLibrary.Delay` 0.2)
  (`PrimitiveComponent.SetMaterial` (`self.Mesh`) 0 null))

(event `ai부활`
  (`self.PlayAnimMontage` "/Game/CANNONSHOOTER/montage/cannonshooter_death_Montage.cannonshooter_death_Montage")
  (`KismetSystemLibrary.Delay` 1.5)
  (`ActorComponent.K2_DestroyComponent` (`self.Mesh`))
  (bind _returnvalue (`|SpawnActorFromClass` "/Game/AI/Aiblade.Aiblade_C" (`self.GetTransform`) "Undefined" "OverrideRootScale" null null))
  (`Controller.Possess` (`GameplayStatics.GetPlayerController` 0) _returnvalue)
  (`ActorComponent.K2_DestroyComponent` (`self.CapsuleComponent`)))

(fn `UpdateRotByMoveKey`
  (params (IsPressRightKey :type Boolean)))

(fn `UserConstructionScript`)

(fn `새 함수`)