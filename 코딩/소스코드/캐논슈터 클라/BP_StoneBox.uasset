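; BP_StoneBox is a breakable box actor that reacts to overlaps on its Box component.
; A BP_FallingStone2 with ComponentCollision set destroys it immediately, spawning a collision effect and playing a destruction sound at the box's location.
; Otherwise, an overlapping BladeBP2 destroys it after a short delay, without effect or sound.
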(event `self.Box.OnComponentBeginOverlap`
  (params (OverlappedComponent :type "PrimitiveComponent Object Reference") (OtherActor :type "Actor Object Reference") (OtherComp :type "PrimitiveComponent Object Reference") (OtherBodyIndex :type Integer) (bFromSweep :type Boolean) (SweepResult :type "HitResult Structure (by ref)"))
  (bind _returnvalue (`SceneComponent.K2_GetComponentLocation` (`self.Box`)))
  (bind _asbp_falling_stone_2 (cast `/Game/BLUEPRINT/BP_FallingStone2` OtherActor)
    (:`then`
      (if (`/Game/BLUEPRINT/BP_FallingStone2.Component Collision` _asbp_falling_stone_2)
        (bind _returnvalue_2 (`NiagaraFunctionLibrary.SpawnSystemAtLocation` "/Game/Assets/VFX/Niagara/FX_stonebox_collision.FX_stonebox_collision" _returnvalue))
        (`GameplayStatics.PlaySoundAtLocation` "/Game/Assets/Sound/Others/destroy_stonebox.destroy_stonebox" _returnvalue (struct) 1.0 1.0 0.0 null null null null)
        (`self.K2_DestroyActor`)
        (`ActorComponent.SetAutoActivate` _returnvalue_2 false)
        (else
          (cast `/Game/BLADE/BladeBP2` OtherActor :!label _label)
          (`KismetSystemLibrary.Delay` 3.0)
          (`self.K2_DestroyActor`))))
    (:`CastFailed`
      (goto _label))))

(fn `UserConstructionScript`)