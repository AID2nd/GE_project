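; BP_TestDamage is a floating damage-number actor that displays a value with a TextRender component.
; SetDamegeText rounds the damage down to an integer and sets it as the text.
; On BeginPlay, a timeline's vector track drives the text's vertical offset from the spawn location (Z) and its X/Y scale (Y channel).
; The actor destroys itself when the timeline finishes.
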(event `self.ReceiveBeginPlay`
  (bind _textrender (`self.TextRender`))
  (set `self.Start Pos` (`self.K2_GetActorLocation`))
  (bind (_direction `_새_트랙_0`) (`Timeline|DamageTextTimeLine`)
    (:`Update`
      (bind _y (.y `_새_트랙_0`))
      (`SceneComponent.K2_SetWorldLocation` (`self.TextRender`) (+ (`self.Start Pos`) (`KismetMathLibrary.MakeVector` 0.0 0.0 (.z `_새_트랙_0`))) false false)
      (`TextRenderComponent.SetXScale` _textrender _y)
      (`TextRenderComponent.SetYScale` _textrender _y))
    (:`Finished`
      (`self.K2_DestroyActor`))))

(fn `Set DamegeText`
  (params (Damage :type "Float (double-precision)"))
  (`TextRenderComponent.K2_SetText` (`self.TextRender`) (`KismetTextLibrary.Conv_IntToText` (`KismetMathLibrary.FFloor` Damage))))

(fn `UserConstructionScript`)