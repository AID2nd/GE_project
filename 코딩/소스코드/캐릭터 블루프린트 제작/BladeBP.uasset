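; Player-controlled Blade character for a side-scroll game, with movement, jump, dash montage and a three-hit melee combo.
; Animation-driven events advance the buffered combo and toggle the attack capsule, which damages overlapping characters with a different tag.
; Damage and Tick-polled potion healing update the GameInstance's HP bar, with a brief material flash on hit.
; Death prints jump and attack stats, destroys the actor and spawns a Bladeai at its transform.
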(event `self.ReceiveBeginPlay`
  (`PlayerController.SetViewTargetWithBlend` (`GameplayStatics.GetPlayerController` 0) (`self.Cam`) 0.0 "VTBlend_Linear" 0.0 false)
  (bind _asside_scroll_game_instance (cast `/Game/Blueprints/SideScrollGameInstance` (`GameplayStatics.GetGameInstance`)))
  (set `self.SideScrollGameInsRef` _asside_scroll_game_instance))

(event `self.ReceiveTick`
  (params (DeltaSeconds :type "Float (single-precision)"))
  (bind _asboam_bp (cast `/Game/item/boam_BP` (`self.portion`)))
  (if (`/Game/item/boam_BP.isGetPortion` _asboam_bp)
    (bind _output_get (set `self.Hp` (+ (`self.Hp`) 10.0)))
    (`/Game/Blueprints/Widgets/GamePlayMain_2.Update_HeroHPBar` (`/Game/Blueprints/SideScrollGameInstance.gameWidget2` (`self.SideScrollGameInsRef`)) (`self.Hp`) (`self.MaxHp`))
    (`KismetSystemLibrary.PrintText` (`KismetTextLibrary.Conv_DoubleToText` _output_get "HalfToEven"))))

(event `InputAxis|LeftRight`
  (params (AxisValue :type "Float (single-precision)"))
  (if (not (`self.IsAttacking`))
    (`self.AddMovementInput` (0.0 1.0 0.0) AxisValue)))

(event `Key|LeftShift`
  (params (Key :type "Key Structure"))
  (:`Pressed`
    (`self.PlayAnimMontage` "/Game/BLADE/Animation/BLADE_DASH_Montage.BLADE_DASH_Montage")))

(event `InputAxis|ForwardBackward`
  (params (AxisValue :type "Float (single-precision)"))
  (if (not (`self.IsAttacking`))
    (`self.AddMovementInput` (1.0 0.0 0.0) AxisValue)))

(event `Key|LeftMouseButton`
  (params (Key :type "Key Structure"))
  (:`Pressed`
    (if (`self.IsAttacking`)
      (set `self.Is Go Next Combo` true)
      (else
        (set `self.IsAttacking` true)
        (`self.PlayAnimMontage` "/Game/BLADE/montage/blade_attack1_Montage.blade_attack1_Montage")
        (`self.UpdateRotByMoveKey` (`self.Is Press Right Key`))
        (set `self.Attack Count` (+ (`self.Attack Count`) 1))))))

(event `OnAnimEnd_Attack`
  (set `self.IsAttacking` false)
  (set `self.Is Go Next Combo` false)
  (set `self.Combo Count` 0))

(event `OnAnim_CheckNextCombo`
  (if (`self.Is Go Next Combo`)
    (set `self.Is Go Next Combo` false)
    (bind _output_get (set `self.Combo Count` (+ (`self.Combo Count`) 1)))
    (switch `int` _output_get
      (:`1`
        (set `self.Attack Count` (+ (`self.Attack Count`) 1))
        (`self.PlayAnimMontage` "/Game/BLADE/montage/blade_attack2_Montage.blade_attack2_Montage"))
      (:`2`
        (set `self.Attack Count` (+ (`self.Attack Count`) 1))
        (`self.PlayAnimMontage` "/Game/BLADE/montage/blade_attack3_Montage.blade_attack3_Montage")))
    (`self.UpdateRotByMoveKey` (`self.Is Press Right Key`))))

(event `Key|SpaceBar`
  (params (Key :type "Key Structure"))
  (:`Pressed`
    (if (`NavMovementComponent.IsFalling` (`self.CharacterMovement`))
      _
      (elif (not (`self.IsAttacking`))
        (`self.Jump`)
        (`self.PlayAnimMontage` "/Game/BLADE/montage/BLADE_JUMP_Montage.BLADE_JUMP_Montage"))))
  (:`Released`
    (`self.StopJumping`)))

(event `self.OnLanded`
  (params (Hit :type "HitResult Structure (by ref)"))
  (`self.StopAnimMontage` "/Game/BLADE/montage/BLADE_JUMP_Montage.BLADE_JUMP_Montage")
  (set `self.jumpCount` (+ (`self.jumpCount`) 1)))

(event `self.Capsule.OnComponentBeginOverlap`
  (params (OverlappedComponent :type "PrimitiveComponent Object Reference") (OtherActor :type "Actor Object Reference") (OtherComp :type "PrimitiveComponent Object Reference") (OtherBodyIndex :type Integer) (bFromSweep :type Boolean) (SweepResult :type "HitResult Structure (by ref)"))
  (if (!= OtherActor self)
    (if (!= (`|GetArrayItem` (`self.Tags`)) (`|GetArrayItem` (`Actor.Tags` OtherActor)))
      (if (== (`|GetArrayItem` (`ActorComponent.ComponentTags` OtherComp)) "Character")
        (`GameplayStatics.ApplyDamage` OtherActor (`self.Atk`) null self)
        (set `self.colAttackcount` (+ (`self.colAttackcount`) 1))))))

(event `OnCollStart_Attack`
  (`PrimitiveComponent.SetCollisionEnabled` (`self.Capsule`) "QueryAndPhysics"))

(event `OnCollEnd_Attack`
  (`PrimitiveComponent.SetCollisionEnabled` (`self.Capsule`) "NoCollision"))

(event `self.ReceiveAnyDamage`
  (params (Damage :type "Float (single-precision)") (DamageType :type "DamageType Object Reference") (InstigatedBy :type "Controller Object Reference") (DamageCauser :type "Actor Object Reference"))
  (bind _output_get (set `self.Hp` (- (`self.Hp`) Damage)))
  (`/Game/Blueprints/Widgets/GamePlayMain_2.Update_HeroHPBar` (`/Game/Blueprints/SideScrollGameInstance.gameWidget2` (`self.SideScrollGameInsRef`)) (`self.Hp`) (`self.MaxHp`))
  (`self.ChangeDamageColor`)
  (if (<= _output_get 0.0)
    (`self.PlayAnimMontage` "/Game/BLADE/montage/BLADE_DEATH_Montage.BLADE_DEATH_Montage")
    (set `self.IsDeath` true)
    (`KismetSystemLibrary.PrintText` (`|FormatText` "점프애니메이션 : {n}, 공격횟수  : {n2},  공격성공횟수 : { n3}" (`self.jumpCount`) (`self.Attack Count`) (`self.colAttackcount`)))
    (`self.DisableInput` null)
    (`self.K2_DestroyActor`)
    (`|SpawnActorFromClass` "/Game/AI/bladeai.bladeai_C" (`self.GetTransform`) "AlwaysSpawn" "OverrideRootScale" null null)
    (bind _asside_scroll_game_instance (cast `/Game/Blueprints/SideScrollGameInstance` (`GameplayStatics.GetGameInstance`)))
    (set `self.SideScrollGameInsRef` _asside_scroll_game_instance)))

(event `ChangeDamageColor`
  (`PrimitiveComponent.SetMaterial` (`self.Mesh`) 0 "/Game/Mesh/Paladin/Paladin_MAT_Inst.Paladin_MAT_Inst")
  (`KismetSystemLibrary.Delay` 0.2)
  (`PrimitiveComponent.SetMaterial` (`self.Mesh`) 0 "/Game/InfinityBladeIceLands/Maps/LevelContent/Architecture/M_1Meter_01.M_1Meter_01"))

(fn `UpdateRotByMoveKey`
  (params (IsPressRightKey :type Boolean)))

(fn `UserConstructionScript`)